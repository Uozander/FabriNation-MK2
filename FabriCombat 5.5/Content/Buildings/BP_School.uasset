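; BP_School is a school building that houses citizens nearby and adjusts the player's Wealth every second by worker income minus fixed upkeep.
; Shortly after BeginPlay it destroys itself if it overlaps a BP_Industry whose material is not MAT_Trans.
; CE_HomeSpawn traces in a random cardinal direction, then spawns a BP_Residential, tiers up one below max level, or destroys the citizen.
; Each housed citizen increments Workers and the controller's Citizens.
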(event Custom|CE_HomeSpawn
  (params (Citizen :type Actor%20Object%20Reference))
  (Variables|Default|SetCitizen Citizen)
  (switch int (Math|Random|RandomInteger 4)
    (:0
      (CallFunction|SpawnHome (Variables|Default|GetNorth) (Variables|Default|GetCitizen)))
    (:1
      (CallFunction|SpawnHome (Variables|Default|GetSouth) (Variables|Default|GetCitizen)))
    (:2
      (CallFunction|SpawnHome (Variables|Default|GetWest) (Variables|Default|GetCitizen)))
    (:3
      (CallFunction|SpawnHome (Variables|Default|GetEast) (Variables|Default|GetCitizen)))))

(event EventBeginPlay
  (bind _overlappingactors (Collision|GetOverlappingActors "/Game/Buildings/BP_Industry.BP_Industry_C" :!class /Script/Engine.Actor))
  (bind _workers (Variables|Default|GetWorkers))
  (Utilities|FlowControl|Sequence
    (:then_0
      (Utilities|FlowControl|Delay 0.1)
      (if (not (Utilities|Array|IsEmpty _overlappingactors))
        (Utilities|IsValid (Variables|Default|GetBox)
          (:Is%20Valid
            (for _array_element _overlappingactors
              (if (== (Utilities|GetClass _array_element) "/Game/Buildings/BP_Industry.BP_Industry_C")
                (bind _asbp_industry (Utilities|Casting|CastToBP_Industry _array_element))
                (Utilities|IsValid (Variables|/Game/Buildings/BP_Industry.BP_Industry_C|GetStructure _asbp_industry)
                  (:Is%20Valid
                    (if (not (== (Rendering|Material|GetMaterial (Variables|/Game/Buildings/BP_Industry.BP_Industry_C|GetStructure _asbp_industry) 0) "/Game/Materials/MAT_Trans.MAT_Trans"))
                      (Actor|DestroyActor))))))))))
    (:then_1
      (Utilities|FlowControl|Delay 1.0 :!label _label)
      (bind _asbp_top_down_controller (Utilities|Casting|CastToBP_TopDownController (Game|GetPlayerController 0)))
      (Variables|/Game/TopDown/Blueprints/BP_TopDownController.BP_TopDownController_C|SetWealth _asbp_top_down_controller (- (+ (Variables|/Game/TopDown/Blueprints/BP_TopDownController.BP_TopDownController_C|GetWealth _asbp_top_down_controller) (* _workers 12)) 48.0))
      (Development|PrintString (Utilities|String|ToString(Integer) _workers))
      (goto _label))))

(fn ConstructionScript)

(fn SpawnHome
  (params (Direction :type Vector) (Citizen :type Actor%20Object%20Reference))
  (bind _structure (Variables|Default|GetStructure))
  (bind _returnvalue (Transformation|GetWorldLocation _structure))
  (bind _returnvalue_2 (+ _returnvalue Direction))
  (bind _returnvalue_3 (- _returnvalue_2 "0.000000,0.000000,50.000000"))
  (bind (_outhit _returnvalue_4) (Collision|LineTraceByChannel (+ _returnvalue "0.000000,0.000000,50.000000") _returnvalue_2 "TraceTypeQuery1" false 0 "ForOneFrame"))
  (if _returnvalue_4
    (if (== (Utilities|GetClass (.HitActor (Collision|BreakHitResult _outhit))) "/Game/Buildings/BP_Residential.BP_Residential_C")
      (bind _asbp_residential (Utilities|Casting|CastToBP_Residential (.HitActor (Collision|BreakHitResult _outhit))))
      (if (>= (Variables|/Game/Buildings/BP_Residential.BP_Residential_C|GetLevel _asbp_residential) 5)
        (Actor|DestroyActor Citizen)
        (else
          (Default|CETierUp _asbp_residential Citizen)
          (Variables|Default|SetWorkers (+ (Variables|Default|GetWorkers) 1) :!label _label)
          (bind _asbp_top_down_controller (Utilities|Casting|CastToBP_TopDownController (Game|GetPlayerController 0)))
          (Variables|/Game/TopDown/Blueprints/BP_TopDownController.BP_TopDownController_C|SetCitizens _asbp_top_down_controller (+ (Variables|/Game/TopDown/Blueprints/BP_TopDownController.BP_TopDownController_C|GetCitizens _asbp_top_down_controller) 1.0))))
      (else
        (Actor|DestroyActor Citizen)))
    (else
      (Game|SpawnActorfromClass "/Game/Buildings/BP_Residential.BP_Residential_C" (Math|Transform|MakeTransform _returnvalue_3 "0, 0, 0" "1.000000,1.000000,1.000000") "Undefined" "MultiplyWithRoot" 0 0)
      (bind _asbp_citizen (Utilities|Casting|CastToBP_Citizen Citizen))
      (Variables|/Game/Units/BP_Citizen.BP_Citizen_C|SetHome%20Location _asbp_citizen _returnvalue_3)
      (goto _label))))