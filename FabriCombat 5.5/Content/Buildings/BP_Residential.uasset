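; Residential building that houses citizens, growing in tiers and spreading into neighboring plots.
; Tiering up sets the citizen's home, notifies its workplace and reveals another structure mesh, with upgrade events raising the tier cap.
; At the cap, a random-direction line trace spawns a new residence, passes the citizen to the one hit, or destroys the citizen if otherwise blocked.
; Shortly after BeginPlay, it destroys itself if overlapping industry.
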(event Custom|CE_HomeSpawn
  (params (Citizen :type Actor%20Object%20Reference))
  (Variables|Default|SetCitizen Citizen)
  (switch int (Math|Random|RandomInteger 4)
    (:0
      (CallFunction|SpawnHome (Variables|Default|GetCitizen) (Variables|Default|GetNorth)))
    (:1
      (CallFunction|SpawnHome (Variables|Default|GetCitizen) (Variables|Default|GetSouth)))
    (:2
      (CallFunction|SpawnHome (Variables|Default|GetCitizen) (Variables|Default|GetWest)))
    (:3
      (CallFunction|SpawnHome (Variables|Default|GetCitizen) (Variables|Default|GetEast)))))

(event Custom|CE_TierUp
  (params (Citizen :type Actor%20Object%20Reference))
  (if (>= (Variables|Default|GetLevel) (Variables|Default|GetMax%20Tier))
    (CallFunction|CEHomeSpawn Citizen)
    (else
      (bind _asbp_citizen (Utilities|Casting|CastToBP_Citizen Citizen))
      (Variables|/Game/Units/BP_Citizen.BP_Citizen_C|SetHome%20Location _asbp_citizen (Transformation|GetActorLocation))
      (bind _output_get (Variables|Default|SetLevel (+ (Variables|Default|GetLevel) 1)))
      (Default|CEWorkerUP (Variables|/Game/Units/BP_Citizen.BP_Citizen_C|GetWork _asbp_citizen))
      (switch int _output_get
        (:2
          (Rendering|SetVisibility (Variables|Default|GetBase_Structure1) true true))
        (:3
          (Rendering|SetVisibility (Variables|Default|GetBase_Structure2) true true))
        (:4
          (Rendering|SetVisibility (Variables|Default|GetBase_Structure3) true true))))))

(event Custom|CE_Upgrade_3
  (Variables|Default|SetMax%20Tier (+ (Variables|Default|GetMax%20Tier) 1))
  (Variables|Default|SetUpgrade3? true))

(event Custom|CE_Upgrade_1
  (Variables|Default|SetMax%20Tier (+ (Variables|Default|GetMax%20Tier) 1))
  (Variables|Default|SetUpgrade1? true))

(event Custom|CE_Upgrade_2
  (Variables|Default|SetMax%20Tier (+ (Variables|Default|GetMax%20Tier) 1))
  (Variables|Default|SetUpgrade2? true))

(event EventBeginPlay
  (bind _overlappingactors (Collision|GetOverlappingActors "/Game/Buildings/BP_Industry.BP_Industry_C" :!class /Script/Engine.Actor))
  (Variables|Default|SetResidential%20Name (Utilities|SetName))
  (Rendering|SetVisibility (Variables|Default|GetBase_Structure2) false true)
  (Utilities|FlowControl|Delay 0.1)
  (if (not (Utilities|Array|IsEmpty _overlappingactors))
    (Utilities|IsValid (Variables|Default|GetBox)
      (:Is%20Valid
        (for _array_element _overlappingactors
          (if (== (Utilities|GetClass _array_element) "/Game/Buildings/BP_Industry.BP_Industry_C")
            (Actor|DestroyActor)))))))

(fn ConstructionScript)

(fn SpawnHome
  (params (Citizen :type Actor%20Object%20Reference) (Direction :type Vector))
  (bind _structure_0 (Variables|Default|GetStructure-0))
  (bind _returnvalue (Transformation|GetWorldLocation _structure_0))
  (bind _returnvalue_2 (+ _returnvalue Direction))
  (bind (_outhit _returnvalue_3) (Collision|LineTraceByChannel _returnvalue _returnvalue_2 "TraceTypeQuery1" false 0 "None"))
  (if _returnvalue_3
    (if (== (Utilities|GetClass (.HitActor (Collision|BreakHitResult _outhit))) "BP_Residential_C")
      (bind _asbp_residential (Utilities|Casting|CastToBP_Residential (.HitActor (Collision|BreakHitResult _outhit))))
      (if (>= (Variables|BP_Residential_C|GetLevel _asbp_residential) (Variables|BP_Residential_C|GetMax%20Tier _asbp_residential))
        (CallFunction|CEHomeSpawn _asbp_residential Citizen)
        (else
          (CallFunction|CETierUp _asbp_residential Citizen)))
      (else
        (Actor|DestroyActor Citizen)))
    (else
      (Variables|Default|SetSpawn%20Location%20X (Math|Conversions|ToFloat(Integer) (* (Math|Float|Round (/ (.x (.Location (Collision|BreakHitResult _outhit))) 2.5e+02)) 250)))
      (Variables|Default|SetSpawn%20Location%20Y (Math|Conversions|ToFloat(Integer) (* (Math|Float|Round (/ (.y (.Location (Collision|BreakHitResult _outhit))) 2.5e+02)) 250)))
      (Game|SpawnActorfromClass "BP_Residential_C" (Math|Transform|MakeTransform _returnvalue_2 "0, 0, 0" "1.000000,1.000000,1.000000") "Undefined" "MultiplyWithRoot" 0 0)
      (Variables|Default|SetLevel (+ (Variables|Default|GetLevel) 1))
      (bind _asbp_citizen (Utilities|Casting|CastToBP_Citizen Citizen))
      (Variables|/Game/Units/BP_Citizen.BP_Citizen_C|SetHome%20Location _asbp_citizen _returnvalue_2)
      (return))))

(fn SpawnHome
  (params (Citizen :type Actor%20Object%20Reference))
  (bind _base_structure1 (Variables|Default|GetBase_Structure1))
  (bind _returnvalue (Transformation|GetWorldLocation _base_structure1))
  (bind _returnvalue_2 (+ _returnvalue ""))
  (bind _returnvalue_3 (- _returnvalue_2 "0.000000,0.000000,50.000000"))
  (bind (_outhit _returnvalue_4) (Collision|LineTraceByChannel (+ _returnvalue "0.000000,0.000000,50.000000") _returnvalue_2 "TraceTypeQuery1" false 0 "None"))
  (if _returnvalue_4
    (if (== (Utilities|GetClass (.HitActor (Collision|BreakHitResult _outhit))) "BP_Residential_C")
      (bind _asbp_residential (Utilities|Casting|CastToBP_Residential (.HitActor (Collision|BreakHitResult _outhit))))
      (if (>= (Variables|BP_Residential_C|GetLevel _asbp_residential) 5)
        (Actor|DestroyActor 0)
        (else
          (CallFunction|CETierUp _asbp_residential 0)))
      (else
        (Actor|DestroyActor 0)))
    (else
      (Game|SpawnActorfromClass "BP_Residential_C" (Math|Transform|MakeTransform _returnvalue_3 "0, 0, 0" "1.000000,1.000000,1.000000") "Undefined" "MultiplyWithRoot" 0 0)
      (bind _asbp_citizen (Utilities|Casting|CastToBP_Citizen Citizen))
      (Variables|/Game/Units/BP_Citizen.BP_Citizen_C|SetHome%20Location _asbp_citizen _returnvalue_3))))