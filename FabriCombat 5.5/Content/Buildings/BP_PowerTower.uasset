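; Power tower building whose only live event logic is demolition.
; CE_Demo and Demolish disable cube collision, spawn BP_DEMO_Ind, send the player controller a power-destroyed message and destroy the tower.
; All other events are empty; disconnected industry logic for coal-to-steel production, upgrades, trucks, upkeep and adjacency tubes never runs.
; SpawnHome and CheckAdjacent use directional line traces but are only called from that dead logic.
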(event Custom|CE_HomeSpawn
  (params (Citizen :type Actor%20Object%20Reference)))

(event Custom|CE_Work)

(event Custom|CE_WorkerUP)

(event Custom|CE_Deliver
  (params (Delivery :type STCT%20Resource%20Structure)))

(event Custom|CE_Truck)

(event Custom|CE_Upgrade_2)

(event Custom|CE_Upgrade_1)

(event Custom|CE_Demo
  (Collision|SetCollisionEnabled (Variables|Default|GetCube7) "NoCollision")
  (Game|SpawnActorfromClass "/Game/Buildings/BP_DEMO_Ind.BP_DEMO_Ind_C" (Transformation|GetActorTransform self) "Undefined" "MultiplyWithRoot" 0 0)
  (Class|BPIInteract|PowerDestroyed(Message) (Game|GetPlayerController 0))
  (Actor|DestroyActor))

(event Custom|CE_Upgrade_3)

(event EventBeginPlay)

(event EventDemolish
  (Collision|SetCollisionEnabled (Variables|Default|GetCube7) "NoCollision")
  (Game|SpawnActorfromClass "/Game/Buildings/BP_DEMO_Ind.BP_DEMO_Ind_C" (Transformation|GetActorTransform self) "Undefined" "MultiplyWithRoot" 0 0)
  (Class|BPIInteract|PowerDestroyed(Message) (Game|GetPlayerController 0))
  (Actor|DestroyActor))

(fn ConstructionScript)

(fn SpawnHome
  (params (Direction :type Vector) (Citizen :type Actor%20Object%20Reference))
  (bind _structure (Variables|Default|GetStructure))
  (bind _returnvalue (Transformation|GetWorldLocation _structure))
  (bind _returnvalue_2 (+ _returnvalue Direction))
  (bind _returnvalue_3 (- _returnvalue_2 "0.000000,0.000000,50.000000"))
  (bind (_outhit _returnvalue_4) (Collision|LineTraceByChannel (+ _returnvalue "0.000000,0.000000,50.000000") _returnvalue_2 "TraceTypeQuery1" false 0 "None"))
  (if _returnvalue_4
    (if (== (Utilities|GetClass (.HitActor (Collision|BreakHitResult _outhit))) "/Game/Buildings/BP_Residential.BP_Residential_C")
      (bind _asbp_residential (Utilities|Casting|CastToBP_Residential (.HitActor (Collision|BreakHitResult _outhit))))
      (if (>= (Variables|/Game/Buildings/BP_Residential.BP_Residential_C|GetLevel _asbp_residential) (Variables|/Game/Buildings/BP_Residential.BP_Residential_C|GetMax%20Tier _asbp_residential))
        (Default|CEHomeSpawn _asbp_residential Citizen)
        (else
          (Default|CETierUp _asbp_residential Citizen)))
      (else
        (Actor|DestroyActor Citizen)))
    (else
      (Game|SpawnActorfromClass "/Game/Buildings/BP_Residential.BP_Residential_C" (Math|Transform|MakeTransform _returnvalue_3 "0, 0, 0" "1.000000,1.000000,1.000000") "Undefined" "MultiplyWithRoot" 0 0)
      (bind _asbp_citizen (Utilities|Casting|CastToBP_Citizen Citizen))
      (Variables|/Game/Units/BP_Citizen.BP_Citizen_C|SetHome%20Location _asbp_citizen _returnvalue_3))))

(fn CheckAdjacent
  (params (Direction :type Vector))
  (bind _structure (Variables|Default|GetStructure))
  (bind _returnvalue (Transformation|GetWorldLocation _structure))
  (bind _outhit (Collision|LineTraceByChannel (+ _returnvalue "0.000000,0.000000,50.000000") (+ _returnvalue Direction) "TraceTypeQuery1" false 0 "None"))
  (return (== (Utilities|GetClass (.HitActor (Collision|BreakHitResult _outhit))) "/Game/Buildings/BP_Industry.BP_Industry_C")))