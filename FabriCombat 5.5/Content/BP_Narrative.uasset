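; Narrative manager that advances the game's numbered story steps in sequence and drives the Mission 1 to Mission 2 transition.
; Each step typically plays a random voice line from its dialogue array and updates quest text in the WDG_Narrative widget.
; Step 6 wipes gameplay actors, runs a timed transition, loads Mission_2 as a level instance and repopulates citizens.
; Steps 9–11 trigger escalating enemy waves, each auto-advancing after a delay.
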(event Custom|CE_Narrative
  (params (Sound%20Array :type Array%20of%20Sound%20Wave%20Object%20References))
  (Audio|PlaySound2D (Utilities|Array|Get(acopy) Sound%20Array (Math|Random|RandomInteger (Utilities|Array|Length Sound%20Array))) 1.0 1.0 0.0 0 0)
  (Default|NarrUIUpdate (Variables|Default|GetNarrWDG) (Utilities|Array|Get(acopy) (Variables|Default|GetQuest) (+ (Variables|Default|GetEvent) 1)) (Utilities|Array|Get(acopy) (Variables|Default|GetContext) (+ (Variables|Default|GetEvent) 1))))

(event Custom|CE_Mission%20END
  (bind _dial_6 (Variables|Default|GetDIAL_6))
  (bind _dial_lt (Variables|Default|GetDIAL_LT))
  (CallFunction|CEWipe)
  (Utilities|FlowControl|DoOnce false
    (:Completed
      (Viewport|RemoveAllWidgets)
      (UserInterface|Viewport|AddtoViewport (Variables|Default|GetNarrWDG) 0)
      (Default|CEMission1Transition (Variables|Default|GetNarrWDG))
      (Audio|PlaySound2D (Utilities|Array|Get(acopy) _dial_lt (Math|Random|RandomInteger (Utilities|Array|Length _dial_lt))) 1.0 1.0 0.0 0 0)
      (Utilities|FlowControl|Delay 2.0)
      (Audio|PlaySound2D "/Game/Narrative/Voice_Lines/Jane/Jane_RBT_Earth__5_.Jane_RBT_Earth__5_" 1.0 1.0 0.0 0 0)
      (Utilities|FlowControl|Delay 3.637)
      (Audio|PlaySound2D "/Game/Narrative/Voice_Lines/Jane/Jane_SUPDAY.Jane_SUPDAY" 1.0 1.0 0.0 0 0)
      (Utilities|FlowControl|Delay 1.063)
      (Audio|PlaySound2D (Utilities|Array|Get(acopy) _dial_6 (Math|Random|RandomInteger (Utilities|Array|Length _dial_6))) 1.0 1.0 0.0 0 0)
      (Utilities|FlowControl|Delay 1.5)
      (Viewport|RemoveAllWidgets)
      (Class|LevelStreamingDynamic|LoadLevelInstance "Mission_2" "0.000000,0.000000,-312.000000" "0, 0, 0" "" 0 false)
      (CallFunction|CEReset)
      (bind _returnvalue (UserInterface|CreateWidget "/Game/UI/UI_Base.UI_Base_C"))
      (bind _output_get (Variables|Default|SetBaseUI _returnvalue))
      (UserInterface|Viewport|AddtoViewport _output_get 0)
      (CallFunction|CENarrative (Variables|Default|GetDIAL_6))
      (Input|EnableInput (Game|GetPlayerController 0))
      (bind _outactors (Actor|GetAllActorsOfClasswithTag "/Game/TopDown/Blueprints/BP_Camera.BP_Camera_C" "Play"))
      (for _array_element _outactors
        (Transformation|SetRelativeLocation (Variables|/Game/TopDown/Blueprints/BP_Camera.BP_Camera_C|GetSphere _array_element) (Variables|Default|GetNew%20Location_1) false false))
      (Utilities|FlowControl|Delay 2.5)
      (CallFunction|CEJustdoit)
      (CallFunction|CEReset)
      (bind _returnvalue_2 (Game|SpawnActorfromClass "/Game/BP_Narr_Trigger.BP_Narr_Trigger_C" (Math|Transform|MakeTransform (Variables|Default|GetSpawn%20Transform%20Location_0) "0, 0, 0" "1.000000,1.000000,1.000000") "Undefined" "MultiplyWithRoot" 0 0))
      (Variables|/Game/BP_Narr_Trigger.BP_Narr_Trigger_C|SetNarrative%20# _returnvalue_2 7)
      (bind _returnvalue_3 (Actor|GetActorOfClass "/Game/Blueprints/BP_SPAWN_Citizen.BP_SPAWN_Citizen_C"))
      (if (> (Variables|Default|GetM2copies) 0) :!label _label
        (Default|Kinetic _returnvalue_3 (Variables|Default|GetLocation))
        (Variables|Default|SetM2copies (- (Variables|Default|GetM2copies) 1))
        (Utilities|FlowControl|Delay 0.02)
        (goto _label)
        (else
          (bind _returnvalue_4 (Actor|GetActorOfClass "/Game/Blueprints/BP_SPAWN_Enemy.BP_SPAWN_Enemy_C"))
          (Variables|/Game/Blueprints/BP_SPAWN_Enemy.BP_SPAWN_Enemy_C|SetActive _returnvalue_4 false))))))

(event Custom|CE_Reset
  (UserInterface|Viewport|AddtoViewport (Variables|Default|GetNarrWDG) 0)
  (Default|CEMenuOpen (Variables|Default|GetNarrWDG) (Utilities|Array|Get(acopy) (Variables|Default|GetQuest) (+ (Variables|Default|GetEvent) 1))))

(event Custom|CE_Wipe
  (bind _outactors (Actor|GetAllActorsOfClass "/Game/Blueprints/BP_Citizen2.BP_Citizen2_C"))
  (for _array_element _outactors
    (Actor|DestroyActor _array_element))
  (bind _outactors_2 (Actor|GetAllActorsOfClass "/Game/Blueprints/BP_EnemyAI.BP_EnemyAI_C"))
  (for _array_element_2 _outactors_2
    (Actor|DestroyActor _array_element_2))
  (bind _outactors_3 (Actor|GetAllActorsOfClass "/Game/Buildings/BP_Industry.BP_Industry_C"))
  (for _array_element_3 _outactors_3
    (Actor|DestroyActor _array_element_3))
  (bind _outactors_4 (Actor|GetAllActorsOfClass "/Game/Buildings/BP_PowerTower.BP_PowerTower_C"))
  (for _array_element_4 _outactors_4
    (Actor|DestroyActor _array_element_4))
  (bind _outactors_5 (Actor|GetAllActorsOfClass "/Game/Buildings/BP_Residential.BP_Residential_C"))
  (for _array_element_5 _outactors_5
    (Actor|DestroyActor _array_element_5))
  (bind _outactors_6 (Actor|GetAllActorsOfClass "/Game/Buildings/BP_Clinic.BP_Clinic_C"))
  (for _array_element_6 _outactors_6
    (Actor|DestroyActor _array_element_6)))

(event Custom|CE_Miss2
  ;[0.9635 0.3485 0 0.5] DEP
)

(event Custom|CE_TEST
  (Variables|Default|SetEvent 6)
  (CallFunction|CEMissionEND)
  (Default|CallEndOfMission))

(event Custom|CE_justdoit
  (bind _returnvalue (UserInterface|CreateWidget "/Game/Widgets/WDG_Narrative.WDG_Narrative_C"))
  (Variables|Default|SetNarrWDG _returnvalue)
  (UserInterface|Viewport|AddtoViewport (Variables|Default|GetNarrWDG) 0))

(event EventBeginPlay
  (bind _returnvalue (UserInterface|CreateWidget "/Game/Widgets/WDG_Narrative.WDG_Narrative_C"))
  (Variables|Default|SetNarrWDG _returnvalue)
  (UserInterface|Viewport|AddtoViewport (Variables|Default|GetNarrWDG) 0))

(event EventNarrative
  (params (Event :type Integer))
  (if (== Event (+ (Variables|Default|GetEvent) 1))
    (bind _output_get (Variables|Default|SetEvent Event))
    (switch int _output_get
      (:0
        (CallFunction|CENarrative (Variables|Default|GetDIAL_0)))
      (:1
        (CallFunction|CENarrative (Variables|Default|GetDIAL_1)))
      (:2
        (CallFunction|CENarrative (Variables|Default|GetDIAL_2)))
      (:3
        (CallFunction|CENarrative (Variables|Default|GetDIAL_3)))
      (:4
        (CallFunction|CENarrative (Variables|Default|GetDIAL_4)))
      (:5
        (CallFunction|CENarrative (Variables|Default|GetDIAL_5)))
      (:6
        (Utilities|FlowControl|DoOnce false
          (:Completed
            (Input|DisableInput (Game|GetPlayerController 0))
            (CallFunction|CEMissionEND)
            (Default|CallEndOfMission))))
      (:7
        (CallFunction|CENarrative (Variables|Default|GetDIAL_7)))
      (:8
        (CallFunction|CENarrative (Variables|Default|GetDIAL_8)))
      (:9
        (CallFunction|CENarrative (Variables|Default|GetDIAL_9))
        (Utilities|FlowControl|DoOnce false
          (:Completed
            (bind _returnvalue (Actor|GetActorOfClass "/Game/Blueprints/BP_SPAWN_Enemy.BP_SPAWN_Enemy_C"))
            (Default|CEWave _returnvalue 20)
            (Utilities|FlowControl|Delay 15.0)
            (CallFunction|Narrative 10))))
      (:10
        (CallFunction|CENarrative (Variables|Default|GetDIAL_10))
        (Utilities|FlowControl|DoOnce false
          (:Completed
            (bind _returnvalue_2 (Actor|GetActorOfClass "/Game/Blueprints/BP_SPAWN_Enemy.BP_SPAWN_Enemy_C"))
            (Default|CEWave _returnvalue_2 30)
            (Utilities|FlowControl|Delay 15.0)
            (CallFunction|Narrative 11))))
      (:11
        (CallFunction|CENarrative (Variables|Default|GetDIAL_11))
        (Utilities|FlowControl|DoOnce false
          (:Completed
            (bind _returnvalue_3 (Actor|GetActorOfClass "/Game/Blueprints/BP_SPAWN_Enemy.BP_SPAWN_Enemy_C"))
            (Default|CEWave _returnvalue_3 50)
            (Utilities|FlowControl|Delay 15.0)
            (CallFunction|Narrative 12))))
      (:12
        (CallFunction|CENarrative (Variables|Default|GetDIAL_12)))
      (:13
        (CallFunction|CENarrative (Variables|Default|GetDIAL_13)))
      (:14
        (CallFunction|CENarrative (Variables|Default|GetDIAL_14)))
      (:15
        (CallFunction|CENarrative (Variables|Default|GetDIAL_15)))
      (:16
        (CallFunction|CENarrative (Variables|Default|GetDIAL_16)))
      (:17
        (CallFunction|CENarrative (Variables|Default|GetDIAL_17)))
      (:18
        (CallFunction|CENarrative (Variables|Default|GetDIAL_18)))
      (:19
        (CallFunction|CENarrative (Variables|Default|GetDIAL_19)))
      (:20
        (CallFunction|CENarrative (Variables|Default|GetDIAL_20))))))

(fn ConstructionScript)