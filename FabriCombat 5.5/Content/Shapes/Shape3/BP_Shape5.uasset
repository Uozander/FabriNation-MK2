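; BP_Shape5 procedurally builds a randomly tall stack of floor meshes on BeginPlay, up to a MaxFloors limit.
; Each floor picks a random shape from MeshALL and adds it as a scaled static mesh component with a shared material.
; A transition mesh bridges the previous shape to the new one via per-shape lookup arrays, or repeats at half height when unchanged.
; Older tapering and type-randomisation logic remains disconnected.
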(event Custom|CE_Begin
  (Variables|Default|SetBase_0 (Variables|Default|GetBase))
  (bind _output_get (Variables|Default|SetHeight (+ (Math|Random|RandomInteger (Variables|Default|GetMax%20Floors)) 1)))
  (Utilities|Array|SetArrayElem (Variables|Default|GetEmpty) _output_get false true)
  (for (_ _array_index) (Variables|Default|GetEmpty)
    (if (>= (Variables|Default|GetBase_0) 0.0)
      (CallFunction|CEBuild (Math|Conversions|ToFloat(Integer) _array_index) (Variables|Default|GetType)))))

(event Custom|CE_Build
  (params (Floor :type Float%20%28double-precision%29) (Type :type Integer))
  (bind _typ (CallFunction|Build Floor Floor Type))
  (Variables|Default|SetType _typ))

(event Custom|CE_Floor
  (params (Floor :type Float%20%28double-precision%29) (Object :type Static%20Mesh%20Object%20Reference))
  (bind _multiply (Variables|Default|GetMultiply))
  (bind _base_0 (Variables|Default|GetBase_0))
  (bind _floorheight (Variables|Default|GetFloorHeight))
  (bind _returnvalue (* _base_0 _multiply))
  (bind _returnvalue_2 (AddComponent|AddStaticMeshComponent false (Math|Transform|MakeTransform (Math|Vector|MakeVector 0.0 0.0 (* Floor (* _floorheight 36.015))) (Math|Rotator|MakeRotator 0.0 0.0 0.0) (Math|Vector|MakeVector _returnvalue _returnvalue _floorheight))))
  (Components|StaticMesh|SetStaticMesh _returnvalue_2 Object)
  (Rendering|Material|SetMaterial _returnvalue_2 0 (Variables|Default|GetMaterial)))

(event Custom|CE_Floorgen
  (params (Floor :type Float%20%28double-precision%29))
  (CallFunction|CEFloor Floor (Variables|Default|GetSelection)))

(event Custom|CE_Transition
  (params (Floor :type Float%20%28double-precision%29) (Type :type Integer) (Random :type Integer))
  (if (== Type Random)
    (CallFunction|CETransMesh Floor (Utilities|Array|Get(acopy) (Variables|Default|GetMesh_ALL) Type) 0.5)
    (else
      (switch int Type
        (:0
          (CallFunction|CETransMesh Floor (Utilities|Array|Get(acopy) (Variables|Default|GetMesh_THREE) (- Random 1)) 1.0))
        (:1
          (if (> Random 1)
            (CallFunction|CETransMesh Floor (Utilities|Array|Get(acopy) (Variables|Default|GetMesh_FOUR) (- Random 1)) 1.0)
            (else
              (CallFunction|CETransMesh Floor (Utilities|Array|Get(acopy) (Variables|Default|GetMesh_FOUR) Random) 1.0))))
        (:2
          (if (== Random 3)
            (CallFunction|CETransMesh Floor (Utilities|Array|Get(acopy) (Variables|Default|GetMesh_FIVE) 2) 1.0)
            (else
              (CallFunction|CETransMesh Floor (Utilities|Array|Get(acopy) (Variables|Default|GetMesh_FIVE) Random) 1.0))))
        (:3
          (CallFunction|CETransMesh Floor (Utilities|Array|Get(acopy) (Variables|Default|GetMesh_SIX) Random) 1.0))))))

(event Custom|CE_TransMesh
  (params (Floor :type Float%20%28double-precision%29) (Transition :type Static%20Mesh%20Object%20Reference) (Height%20Scale :type Float%20%28double-precision%29))
  (bind _base_0 (Variables|Default|GetBase_0))
  (bind _floorheight (Variables|Default|GetFloorHeight))
  (bind _multiply (Variables|Default|GetMultiply))
  (bind _returnvalue (* _base_0 _multiply))
  (bind _returnvalue_2 (AddComponent|AddStaticMeshComponent false (Math|Transform|MakeTransform (Math|Vector|MakeVector 0.0 0.0 (+ (* Floor (* _floorheight 36.015)) (* (Variables|Default|GetOffset) 24.01))) (Math|Rotator|MakeRotator 0.0 0.0 0.0) (Math|Vector|MakeVector _returnvalue _returnvalue (* Height%20Scale _floorheight)))))
  (Components|StaticMesh|SetStaticMesh _returnvalue_2 Transition)
  (Rendering|Material|SetMaterial _returnvalue_2 0 (Variables|Default|GetMaterial)))

(event EventBeginPlay
  (CallFunction|CEBegin))

(fn ConstructionScript)

(fn Build
  (params (Floor :type Float%20%28double-precision%29) (Floor2 :type Float%20%28double-precision%29) (Type :type Integer))
  (bind _random (Utilities|Entropy (Variables|Default|GetMesh_ALL)))
  (CallFunction|CETransition Floor Type _random)
  (CallFunction|CEFloorgen Floor2)
  (return _random))