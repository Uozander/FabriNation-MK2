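; BP_Nuke is a nuke explosion actor that flashes a light, expands a blast sphere and damages enemies it hits.
; On BeginPlay, short Delay loops rapidly ramp the PointLight intensity up, then fade it out while the Sphere scales up exponentially.
; Once the light is out, the actor waits briefly and destroys itself.
; Sphere hit events call Damage on any BP_EnemyAI struck, flagged as missile damage.
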(event OnComponentHit(Sphere)
  (params (HitComponent :type Primitive%20Component%20Object%20Reference) (OtherActor :type Actor%20Object%20Reference) (OtherComp :type Primitive%20Component%20Object%20Reference) (NormalImpulse :type Vector :default "0, 0, 0") (Hit :type Hit%20Result%20Structure%20%28by%20ref%29))
  (bind _asbp_enemy_ai (Utilities|Casting|CastToBP_EnemyAI OtherActor))
  (Default|Damage _asbp_enemy_ai "0, 0, 0" true 1))

(event EventBeginPlay
  (bind _pointlight (Variables|Default|GetPointLight))
  (bind _pointlight_2 (Variables|Default|GetPointLight))
  (bind _sphere (Variables|Default|GetSphere))
  (bind _returnvalue (Transformation|GetRelativeTransform _sphere))
  (bind _intensity (Variables|/Script/Engine.LightComponentBase|GetIntensity _pointlight))
  (bind _intensity_2 (Variables|/Script/Engine.LightComponentBase|GetIntensity _pointlight_2))
  (if (<= _intensity 5e+07) :!label _label
    (Rendering|Components|Light|SetIntensity (Variables|Default|GetPointLight) (- _intensity -1e+07))
    (Utilities|FlowControl|Delay 0.01)
    (goto _label)
    (else
      (if (>= _intensity_2 0.0) :!label _label_2
        (Rendering|Components|Light|SetIntensity (Variables|Default|GetPointLight) (- _intensity_2 1.5e+06))
        (Utilities|FlowControl|Delay 0.01)
        (Transformation|SetRelativeTransform _sphere (Math|Transform|MakeTransform (.location _returnvalue) (.rotation _returnvalue) (* (.scale _returnvalue) "1.200000,1.200000,1.200000")) false false)
        (goto _label_2)
        (else
          (Utilities|FlowControl|Delay 3.0)
          (Actor|DestroyActor))))))

(fn ConstructionScript)