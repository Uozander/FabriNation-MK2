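; BP_Truck is a delivery truck that hauls ore to a destination building, then destroys itself.
; CE_Deliver switches on OreNumber to target the last-found train station, or an Industry or NecroT plant chosen by randomly favoring lower stock.
; It turns toward the target and lerps there on timelines rate-scaled by distance and Speed, though the NecroT branch rates a different timeline.
; Arrival hands over the Delivery; no target means immediate destruction.
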(event Custom|CE_Deliver
  (params (Delivery :type STCT%20Resource%20Structure))
  (switch int (.Ore_Number (Utilities|Struct|BreakSTCT_Resource Delivery))
    (:0
      (Variables|Default|SetWork%20Location (Transformation|GetActorLocation))
      (bind _outactors (Actor|GetAllActorsOfClass "/Game/Buildings/BP_TrainStation.BP_TrainStation_C"))
      (if (Utilities|Array|IsEmpty _outactors)
        (Actor|DestroyActor)
        (else
          (for _array_element _outactors
            (bind _output_get (Variables|Default|SetTrainStation _array_element)))
          (bind _output_get_2 (Variables|Default|SetDelivery%20Location (Transformation|GetActorLocation _output_get)))
          (Transformation|SetActorRotation (Math|Rotator|FindLookatRotation (Variables|Default|GetWork%20Location) _output_get_2))
          (Components|Timeline|SetPlayRate (Variables|Default|GetTimeline) (/ 1.0 (/ (Math|Vector|Distance(Vector) (Variables|Default|GetWork%20Location) (Variables|Default|GetDelivery%20Location)) (Variables|Default|GetSpeed))))
          (bind _newtrack_0 (Timeline|Timeline PlayFromStart)
            (:Update
              (Transformation|SetActorLocation (Math|Vector|Lerp(Vector) (Variables|Default|GetWork%20Location) (Variables|Default|GetDelivery%20Location) _newtrack_0) false false))
            (:Finished
              (Default|CEDelivery (Variables|Default|GetTrainStation) Delivery)
              (Actor|DestroyActor))))))
    (:1
      (Variables|Default|SetWork%20Location (Transformation|GetActorLocation))
      (bind _outactors_2 (Actor|GetAllActorsOfClass "/Game/Buildings/BP_Industry.BP_Industry_C"))
      (if (Utilities|Array|IsEmpty _outactors_2)
        (Actor|DestroyActor)
        (else
          (for _array_element_2 _outactors_2
            (if (Utilities|IsValid (Variables|Default|GetDelivery%20Target))
              (if (< (Variables|/Game/Buildings/BP_Industry.BP_Industry_C|GetCoal%20Ore _array_element_2) (Variables|/Game/Buildings/BP_Industry.BP_Industry_C|GetCoal%20Ore (Variables|Default|GetDelivery%20Target)))
                (if (>= (- (Math|Random|RandomFloat) (/ (Variables|/Game/Buildings/BP_Industry.BP_Industry_C|GetCoal%20Ore _array_element_2) 2000)) 0.5)
                  (Variables|Default|SetDelivery%20Target _array_element_2)))
              (else
                (Variables|Default|SetDelivery%20Target _array_element_2))))
          (bind _output_get_3 (Variables|Default|SetDelivery%20Location (Transformation|GetActorLocation (Variables|Default|GetDelivery%20Target))))
          (Transformation|SetActorRotation (Math|Rotator|FindLookatRotation (Variables|Default|GetWork%20Location) _output_get_3))
          (Components|Timeline|SetPlayRate (Variables|Default|GetTimeline_0) (/ 1.0 (/ (Math|Vector|Distance(Vector) (Variables|Default|GetWork%20Location) (Variables|Default|GetDelivery%20Location)) (Variables|Default|GetSpeed))))
          (bind _newtrack_0_2 (Timeline|Timeline_0 PlayFromStart)
            (:Update
              (Transformation|SetActorLocation (Math|Vector|Lerp(Vector) (Variables|Default|GetWork%20Location) (Variables|Default|GetDelivery%20Location) _newtrack_0_2) false false))
            (:Finished
              (Default|CEDeliver (Variables|Default|GetDelivery%20Target) Delivery)
              (Actor|DestroyActor))))))
    (:2
      (Variables|Default|SetWork%20Location (Transformation|GetActorLocation))
      (bind _outactors_3 (Actor|GetAllActorsOfClass "/Game/Buildings/BP_IND_NecroT.BP_IND_NecroT_C"))
      (if (Utilities|Array|IsEmpty _outactors_3)
        (Actor|DestroyActor)
        (else
          (for _array_element_3 _outactors_3
            (if (Utilities|IsValid (Variables|Default|GetNecroT%20Delivery))
              (if (< (Variables|/Game/Buildings/BP_IND_NecroT.BP_IND_NecroT_C|GetNecrotitanium%20Ore _array_element_3) (Variables|/Game/Buildings/BP_IND_NecroT.BP_IND_NecroT_C|GetNecrotitanium%20Ore (Variables|Default|GetNecroT%20Delivery)))
                (if (>= (- (Math|Random|RandomFloat) (/ 0 2000)) 0.5)
                  (Variables|Default|SetNecroT%20Delivery _array_element_3)))
              (else
                (Variables|Default|SetNecroT%20Delivery _array_element_3))))
          (bind _output_get_4 (Variables|Default|SetDelivery%20Location (Transformation|GetActorLocation (Variables|Default|GetNecroT%20Delivery))))
          (Transformation|SetActorRotation (Math|Rotator|FindLookatRotation (Variables|Default|GetWork%20Location) _output_get_4))
          (Components|Timeline|SetPlayRate (Variables|Default|GetTimeline_0) (/ 1.0 (/ (Math|Vector|Distance(Vector) (Variables|Default|GetWork%20Location) (Variables|Default|GetDelivery%20Location)) (Variables|Default|GetSpeed))))
          (bind _newtrack_0_3 (Timeline|Timeline_1 PlayFromStart)
            (:Update
              (Transformation|SetActorLocation (Math|Vector|Lerp(Vector) (Variables|Default|GetWork%20Location) (Variables|Default|GetDelivery%20Location) _newtrack_0_3) false false))
            (:Finished
              (Default|CEDeliver (Variables|Default|GetNecroT%20Delivery) Delivery)
              (Actor|DestroyActor))))))))

(event Collision|EventActorBeginOverlap
  (params (OtherActor :type Actor%20Object%20Reference))
  ;[1 0.5226 0] DEP
)

(fn ConstructionScript)