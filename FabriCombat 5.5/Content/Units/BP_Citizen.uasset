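; BP_Citizen is a simulated city resident that commutes between home and a random BP_Industry, detouring to a random grocery or clinic when food or medical runs low.
; Delay loops decay needs, age the citizen toward random death, and poll road overlap to set mesh and speed multiplier.
; Trips lerp actor location on reversing Timelines paced by SpeedCalc, triggering work or refilling needs on return.
; Upgrade events grant a car or extra speed.
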(event Custom|CE_Upgrade_3
  (Variables|Default|SetSpeed (+ (Variables|Default|GetSpeed) 5e+01))
  (Variables|Default|SetUpgrade3? true))

(event Custom|CE_Upgrade_1
  (Variables|Default|SetCar? true)
  (Variables|Default|SetUpgrade1? true))

(event Custom|CE_Upgrade_2
  (Variables|Default|SetSpeed (+ (Variables|Default|GetSpeed) 5e+01))
  (Variables|Default|SetUpgrade2? true))

(event EventBeginPlay
  (bind _staticmesh (Variables|Default|GetStaticMesh))
  (bind _work_location (Variables|Default|GetWork%20Location))
  (bind _home_location (Variables|Default|GetHome%20Location))
  (bind _work (Variables|Default|GetWork))
  (bind _staticmesh_2 (Variables|Default|GetStaticMesh))
  (Variables|Default|SetAge (+ (Math|Random|RandomInteger 7) 12))
  (Variables|Default|SetCitizen%20Name (Utilities|SetName))
  (Utilities|FlowControl|Sequence
    (:then_0
      (if (Utilities|Array|IsEmpty (Collision|GetOverlappingActors (Variables|Default|GetStaticMesh) "/Game/Tiles/BP_Road.BP_Road_C" :!class /Script/Engine.PrimitiveComponent)) :!label _label
        (Components|StaticMesh|SetStaticMesh _staticmesh "/Game/LevelPrototyping/Meshes/SM_Cube.SM_Cube")
        (Transformation|SetRelativeScale3D _staticmesh "1.000000,1.000000,4.000000")
        (Variables|Default|SetSpeed%20Mult 1.0)
        (elif (Variables|Default|GetCar?)
          (Components|StaticMesh|SetStaticMesh _staticmesh_2 "/Game/Units/FabriTruck2.FabriTruck2")
          (Transformation|SetRelativeScale3D _staticmesh_2 "1.000000,1.000000,1.000000")
          (Variables|Default|SetSpeed%20Mult 4.0)
          (else
            (Variables|Default|SetSpeed%20Mult 1.5))))
      (Utilities|FlowControl|Delay 3.0)
      (goto _label))
    (:then_1
      (Utilities|FlowControl|Sequence
        (:then_0
          (CallFunction|FNWorkFind)
          (Utilities|IsValid (Variables|Default|GetWork)
            (:Is%20Valid
              (Default|CEHomeSpawn (Variables|Default|GetWork) self)
              (Rendering|Material|SetVectorParameterValueonMaterials (Variables|Default|GetStaticMesh1) "Head Color" (Math|Vector|MakeVector (Math|Random|RandomFloat) (Math|Random|RandomFloat) (Math|Random|RandomFloat)))
              (if (or (== (.food (Variables|Default|GetNeeds)) 0) (== (.medical (Variables|Default|GetNeeds)) 0)) :!label _label_2
                (Utilities|FlowControl|Delay 1e+01)
                (goto _label_2)
                (else
                  (Utilities|FlowControl|Delay 1.0 :!label _label_3)
                  (bind _output_get (Variables|Default|SetAgeIncrement (+ (Variables|Default|GetAgeIncrement) 1)))
                  (if (>= _output_get 12)
                    (Variables|Default|SetAgeIncrement 0)
                    (Math|Integer|IncrementInt (.age (Variables|Default|GetNeeds))
                      (:%20%20
                        (Variables|Default|SetNeeds (Utilities|Struct|MakeSCT_Needs (Math|Integer|Clamp(Integer) (- (.food (Variables|Default|GetNeeds)) 1) 0 100) (Math|Integer|Clamp(Integer) (- (.medical (Variables|Default|GetNeeds)) 1) 0 100) 0 (+ (.age (Variables|Default|GetNeeds)) 1)))))
                    (else
                      (Variables|Default|SetNeeds (Utilities|Struct|MakeSCT_Needs (Math|Integer|Clamp(Integer) (- (.food (Variables|Default|GetNeeds)) 1) 0 100) (Math|Integer|Clamp(Integer) (- (.medical (Variables|Default|GetNeeds)) 1) 0 100) 0 (.age (Variables|Default|GetNeeds))))))
                  (if (>= (.age (Variables|Default|GetNeeds)) 80)
                    (if (>= (Math|Random|RandomInteger (.age (Variables|Default|GetNeeds))) 80)
                      (Actor|DestroyActor)
                      (else
                        (goto _label_3)))
                    (else
                      (goto _label_3))))))
            (:Is%20Not%20Valid
              (Actor|DestroyActor))))
        (:then_1
          (if (Utilities|Operators|EqualEqual :A _work_location)
            (Actor|DestroyActor :!label _label_4)
            (elif (== (Math|Vector|Distance(Vector) _work_location _home_location) 0.0)
              (goto _label_4)
              (else
                (if (or (< (.food (Variables|Default|GetNeeds)) 20) (< (.medical (Variables|Default|GetNeeds)) 20)) :!label _label_5
                  (if (< (.food (Variables|Default|GetNeeds)) 20)
                    (bind _outactors (Actor|GetAllActorsOfClass "/Game/Buildings/BP_Grocery.BP_Grocery_C"))
                    (if (== (Utilities|Array|Length _outactors) 0)
                      (Variables|Default|SetCondition false :!label _label_6)
                      (Components|Timeline|SetPlayRate (Variables|Default|GetTimeline) (Utilities|SpeedCalc _home_location))
                      (bind _newtrack_0 (Timeline|Timeline PlayFromStart)
                        (:Update
                          (Transformation|SetActorLocation (Math|Vector|Lerp(Vector) (Variables|Default|GetWork%20Location) (Variables|Default|GetHome%20Location) _newtrack_0) false false))
                        (:Finished
                          (if (Variables|Default|GetCondition)
                            (Utilities|IsValid _work
                              (:Is%20Valid
                                _)
                              (:Is%20Not%20Valid
                                (CallFunction|FNWorkFind)))
                            (Default|CEWork _work)
                            (goto _label_5)
                            (else
                              (Variables|Default|SetCondition true)
                              (Timeline|Timeline ReverseFromEnd)))))
                      (else
                        (for (_array_element _array_index) _outactors
                          (if (== _array_index (Math|Random|RandomInteger (Utilities|Array|Length _outactors)))
                            (bind _output_get_2 (Variables|Default|SetB (Transformation|GetActorLocation _array_element)))))
                        (Variables|Default|SetCondition false)
                        (Components|Timeline|SetPlayRate (Variables|Default|GetTimeline_0) (Utilities|SpeedCalc _output_get_2))
                        (bind _newtrack_2 (Timeline|Timeline_0 PlayFromStart)
                          (:Update
                            (Transformation|SetActorLocation (Math|Vector|Lerp(Vector) (Variables|Default|GetWork%20Location) (Variables|Default|GetB) _newtrack_2) false false))
                          (:Finished
                            (if (Variables|Default|GetCondition)
                              (Variables|Default|SetNeeds (Utilities|Struct|MakeSCT_Needs 100 (.medical (Variables|Default|GetNeeds)) (.education (Variables|Default|GetNeeds)) 0))
                              (goto _label_5)
                              (else
                                (Variables|Default|SetCondition true)
                                (Timeline|Timeline_0 ReverseFromEnd)))))))
                    (elif (< (.medical (Variables|Default|GetNeeds)) 20)
                      (bind _outactors_2 (Actor|GetAllActorsOfClass "/Game/Buildings/BP_Clinic.BP_Clinic_C"))
                      (if (== (Utilities|Array|Length _outactors_2) 0)
                        (goto _label_6)
                        (else
                          (for (_array_element_2 _array_index_2) _outactors_2
                            (if (== _array_index_2 (Math|Random|RandomInteger (Utilities|Array|Length _outactors_2)))
                              (bind _output_get_3 (Variables|Default|SetB (Transformation|GetActorLocation _array_element_2)))))
                          (Variables|Default|SetCondition false)
                          (Components|Timeline|SetPlayRate (Variables|Default|GetTimeline_1) (Utilities|SpeedCalc _output_get_3))
                          (bind _newtrack_0_2 (Timeline|Timeline_1 PlayFromStart)
                            (:Update
                              (Transformation|SetActorLocation (Math|Vector|Lerp(Vector) (Variables|Default|GetWork%20Location) (Variables|Default|GetB) _newtrack_0_2) false false))
                            (:Finished
                              (if (Variables|Default|GetCondition)
                                (Variables|Default|SetNeeds (Utilities|Struct|MakeSCT_Needs (.food (Variables|Default|GetNeeds)) 100 (.education (Variables|Default|GetNeeds)) 0))
                                (goto _label_5)
                                (else
                                  (Variables|Default|SetCondition true)
                                  (Timeline|Timeline_1 ReverseFromEnd)))))))
                      (else
                        (goto _label_5))))
                  (else
                    (goto _label_6)))))))))))

(fn ConstructionScript)

(fn FNWorkFind
  (bind _outactors (Actor|GetAllActorsOfClass "/Game/Buildings/BP_Industry.BP_Industry_C"))
  (if (Utilities|Array|IsEmpty _outactors)
    _
    (else
      (Utilities|IsValid (Utilities|Array|Get(acopy) _outactors (Math|Random|RandomInteger (Utilities|Array|Length _outactors)))
        (:Is%20Valid
          (bind _output_get (Variables|Default|SetWork (Utilities|Array|Get(acopy) _outactors (Math|Random|RandomInteger (Utilities|Array|Length _outactors)))))
          (Variables|Default|SetWork%20Location (Transformation|GetActorLocation _output_get))
          (return))
        (:Is%20Not%20Valid
          _))))
  (Actor|DestroyActor))