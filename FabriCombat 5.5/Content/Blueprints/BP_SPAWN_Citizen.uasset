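; Citizen spawner that creates BP_Citizen2 AI with a Kinetic, Missile or Beam class on request.
; Each request teleports the spawner to a random offset from the given location, spawns the citizen with a bloom effect and sets its class.
; Kinetic builds run on a progress timeline with queued repeats, while Missile and Beam spawn immediately.
; A shared count triggers narrative messages, and a deprecated BeginPlay loop spawns periodically when Active.
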(event Custom|CE_Randomize%20Vector
  (bind _location (Variables|Default|GetLocation))
  (bind _location_2 (Variables|Default|GetLocation))
  (bind _location_3 (Variables|Default|GetLocation))
  (bind _location_4 (Variables|Default|GetLocation))
  (bind (_x _y _z) (Math|Vector|BreakVector _location_2))
  (bind (_x_2 _y_2 _z_2) (Math|Vector|BreakVector _location_3))
  (bind (_x_3 _y_3 _z_3) (Math|Vector|BreakVector _location_4))
  (bind (_x_4 _y_4 _z_4) (Math|Vector|BreakVector _location))
  (switch int (Math|Random|RandomInteger 3)
    (:0
      (Variables|Default|SetSpawn (Math|Vector|MakeVector _x (+ _y 1.5e+02) _z)))
    (:1
      (Variables|Default|SetSpawn (Math|Vector|MakeVector _x_2 (+ _y_2 -1.5e+02) _z_2)))
    (:2
      (Variables|Default|SetSpawn (Math|Vector|MakeVector (+ _x_3 1.5e+02) _y_3 _z_3)))
    (:3
      (Variables|Default|SetSpawn (Math|Vector|MakeVector (+ _x_4 -1.5e+02) _y_4 _z_4)))))

(event Custom|CE_BuildCheck
  (bind _sphere (Variables|Default|GetSphere))
  (bind _returnvalue (Transformation|GetWorldLocation _sphere))
  (if (> (Variables|Default|GetKinetic%20Builds) 0)
    (Variables|Default|SetKinetic%20Builds (+ (Variables|Default|GetKinetic%20Builds) -1))
    (if (Variables|Default|GetBuilding%20Kinetic)
      (Variables|Default|SetKinetic%20Builds (+ (Variables|Default|GetKinetic%20Builds) 1))
      (else
        (Variables|Default|SetBuilding%20Kinetic true)
        (bind _newtrack_1 (Timeline|Timeline PlayFromStart)
          (:Update
            (Variables|Default|SetKinetic%20Build _newtrack_1))
          (:Finished
            (Variables|Default|SetKinetic%20Build 0.0)
            (Variables|Default|SetBuilding%20Kinetic false)
            (Variables|Default|SetLocation (stale EventKinetic Location))
            (CallFunction|CEBuildCheck)
            (CallFunction|CERandomizeVector)
            (Transformation|SetActorLocation self (Variables|Default|GetSpawn) false false)
            (bind _returnvalue_2 (AI|SpawnAIFromClass "/Game/Blueprints/BP_Citizen2.BP_Citizen2_C" "/Game/AI/BT_Citizen.BT_Citizen" _returnvalue "0, 0, 0" false 0))
            (Niagara|SpawnSystematLocation "/Game/Niagara/NS_Bloom.NS_Bloom" _returnvalue)
            (Class|BPIInteract|SetClass(Message) _returnvalue_2)
            (if (<= (Variables|Default|GetCount) 4)
              (Variables|Default|SetCount (+ (Variables|Default|GetCount) 1))
              (else
                (Utilities|FlowControl|DoOnce false
                  (:Completed
                    (bind _returnvalue_3 (Actor|GetActorOfClass "/Game/BP_Narrative.BP_Narrative_C"))
                    (Class|BPIInteract|Narrative(Message) _returnvalue_3 5)))))))))))

(event EventBeginPlay
  ;[1 0.3753 0] DEP
  (if (Variables|Default|GetActive)
    (Utilities|FlowControl|Delay 1e+01 :!label _label)
    (AI|SpawnAIFromClass "/Game/Blueprints/BP_Citizen2.BP_Citizen2_C" "/Game/AI/BT_Citizen.BT_Citizen" (Transformation|GetWorldLocation (Variables|Default|GetSphere)) "0, 0, 0" true 0)
    (goto _label)))

(event EventKinetic
  (params (Location :type Vector :default "0, 0, 0"))
  (bind _sphere (Variables|Default|GetSphere))
  (bind _returnvalue (Transformation|GetWorldLocation _sphere))
  (if (Variables|Default|GetBuilding%20Kinetic)
    (Variables|Default|SetKinetic%20Builds (+ (Variables|Default|GetKinetic%20Builds) 1))
    (else
      (Variables|Default|SetBuilding%20Kinetic true)
      (bind _newtrack_1 (Timeline|Timeline PlayFromStart)
        (:Update
          (Variables|Default|SetKinetic%20Build _newtrack_1))
        (:Finished
          (Variables|Default|SetKinetic%20Build 0.0)
          (Variables|Default|SetBuilding%20Kinetic false)
          (Variables|Default|SetLocation Location)
          (CallFunction|CEBuildCheck)
          (CallFunction|CERandomizeVector)
          (Transformation|SetActorLocation self (Variables|Default|GetSpawn) false false)
          (bind _returnvalue_2 (AI|SpawnAIFromClass "/Game/Blueprints/BP_Citizen2.BP_Citizen2_C" "/Game/AI/BT_Citizen.BT_Citizen" _returnvalue "0, 0, 0" false 0))
          (Niagara|SpawnSystematLocation "/Game/Niagara/NS_Bloom.NS_Bloom" _returnvalue)
          (Class|BPIInteract|SetClass(Message) _returnvalue_2)
          (if (<= (Variables|Default|GetCount) 4)
            (Variables|Default|SetCount (+ (Variables|Default|GetCount) 1))
            (else
              (Utilities|FlowControl|DoOnce false
                (:Completed
                  (bind _returnvalue_3 (Actor|GetActorOfClass "/Game/BP_Narrative.BP_Narrative_C"))
                  (Class|BPIInteract|Narrative(Message) _returnvalue_3 5))))))))))

(event EventMissile
  (params (Location :type Vector :default "0, 0, 0"))
  (bind _sphere (Variables|Default|GetSphere))
  (bind _returnvalue (Transformation|GetWorldLocation _sphere))
  (Variables|Default|SetLocation Location)
  (CallFunction|CERandomizeVector)
  (Transformation|SetActorLocation self (Variables|Default|GetSpawn) false false)
  (bind _returnvalue_2 (AI|SpawnAIFromClass "/Game/Blueprints/BP_Citizen2.BP_Citizen2_C" "/Game/AI/BT_Citizen.BT_Citizen" _returnvalue "0, 0, 0" false 0))
  (Niagara|SpawnSystematLocation "/Game/Niagara/NS_Bloom.NS_Bloom" _returnvalue)
  (Class|BPIInteract|SetClass(Message) _returnvalue_2 1)
  (if (<= (Variables|Default|GetCount) 4)
    (Variables|Default|SetCount (+ (Variables|Default|GetCount) 1))
    (else
      (Utilities|FlowControl|DoOnce false
        (:Completed
          (bind _returnvalue_3 (Actor|GetActorOfClass "/Game/BP_Narrative.BP_Narrative_C"))
          (Class|BPIInteract|Narrative(Message) _returnvalue_3 5))))))

(event EventBeam
  (params (Location :type Vector :default "0, 0, 0"))
  (bind _sphere (Variables|Default|GetSphere))
  (bind _returnvalue (Transformation|GetWorldLocation _sphere))
  (Variables|Default|SetLocation Location)
  (CallFunction|CERandomizeVector)
  (Transformation|SetActorLocation self (Variables|Default|GetSpawn) false false)
  (bind _returnvalue_2 (AI|SpawnAIFromClass "/Game/Blueprints/BP_Citizen2.BP_Citizen2_C" "/Game/AI/BT_Citizen.BT_Citizen" _returnvalue "0, 0, 0" false 0))
  (Niagara|SpawnSystematLocation "/Game/Niagara/NS_Bloom.NS_Bloom" _returnvalue)
  (Class|BPIInteract|SetClass(Message) _returnvalue_2 2)
  (if (<= (Variables|Default|GetCount) 4)
    (Variables|Default|SetCount (+ (Variables|Default|GetCount) 1))
    (else
      (Utilities|FlowControl|DoOnce false
        (:Completed
          (bind _returnvalue_3 (Actor|GetActorOfClass "/Game/BP_Narrative.BP_Narrative_C"))
          (Class|BPIInteract|Narrative(Message) _returnvalue_3 5))))))

(fn ConstructionScript)