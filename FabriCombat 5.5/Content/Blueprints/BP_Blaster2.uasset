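; BP_Blaster2 is an actor, apparently an explosive blaster projectile, that detonates when its Sphere component hits something.
; On hit it plays an explosion sound at the sphere's location, spawns an enlarged Blueprint_Effect_Explosion actor and destroys itself.
; A short delay from BeginPlay destroys it silently if nothing is hit first.
; A DoOnce ricochet sound branch is left unconnected and never runs.
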(event OnComponentHit(Sphere)
  (params (HitComponent :type Primitive%20Component%20Object%20Reference) (OtherActor :type Actor%20Object%20Reference) (OtherComp :type Primitive%20Component%20Object%20Reference) (NormalImpulse :type Vector :default "0, 0, 0") (Hit :type Hit%20Result%20Structure%20%28by%20ref%29))
  (Audio|SpawnSoundatLocation "/Game/StarterContent/Audio/Explosion01.Explosion01" (Transformation|GetWorldLocation (Variables|Default|GetSphere)) "0, 0, 0" 1.0 1.0 0.0 0 0)
  (Game|SpawnActorfromClass "/Game/StarterContent/Blueprints/Blueprint_Effect_Explosion.Blueprint_Effect_Explosion_C" (Math|Transform|MakeTransform "0, 0, 0" "0, 0, 0" "4.000000,4.000000,4.000000") "Undefined" "MultiplyWithRoot" 0 0)
  (Actor|DestroyActor))

(event EventBeginPlay
  (Utilities|FlowControl|Delay 0.5)
  (Actor|DestroyActor))

(fn ConstructionScript)