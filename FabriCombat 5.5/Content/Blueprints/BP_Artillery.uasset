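; Artillery emplacement actor that automatically shells randomly picked "Alien"-tagged BP_EnemyAI actors from BeginPlay onward.
; A one-second loop turns the Sphere toward an enemy, spawns a BP_Proj and lobs it with a pitch-raised impulse, re-rolling the random target between aim and launch.
; Each shot plays a Timeline that flip-flops muzzle flash pairs, then hides them.
; The Box overlap event is empty; its direct-damage cannon logic is disconnected.
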(event OnComponentBeginOverlap(Box)
  (params (OverlappedComponent :type Primitive%20Component%20Object%20Reference) (OtherActor :type Actor%20Object%20Reference) (OtherComp :type Primitive%20Component%20Object%20Reference) (OtherBodyIndex :type Integer) (bFromSweep :type Boolean) (SweepResult :type Hit%20Result%20Structure%20%28by%20ref%29)))

(event Custom|CE_CannonShot
  (bind _sphere (Variables|Default|GetSphere))
  (bind _outactors (Actor|GetAllActorsOfClasswithTag "/Game/Blueprints/BP_EnemyAI.BP_EnemyAI_C" "Alien" :!label _label))
  (Transformation|SetWorldRotation _sphere (Math|Rotator|FindLookatRotation (Transformation|GetWorldLocation (Variables|Default|GetSphere1)) (Transformation|GetActorLocation (Utilities|Array|Get(acopy) _outactors (Math|Random|RandomInteger (Utilities|Array|Length _outactors))))) false false)
  (CallFunction|CEMuzzleShot)
  (bind _returnvalue (Game|SpawnActorfromClass "/Game/Blueprints/BP_Proj.BP_Proj_C" (Math|Transform|MakeTransform (Transformation|GetWorldLocation (Variables|Default|GetSphere1)) (Transformation|GetWorldRotation _sphere) "0.900000,0.900000,0.900000") "AlwaysSpawn" "MultiplyWithRoot" 0 0))
  (Physics|AddImpulse (Variables|/Game/Blueprints/BP_Proj.BP_Proj_C|GetArtillery%20Shell _returnvalue) (* (Math|Vector|GetForwardVector (Math|Rotator|MakeRotator (.Roll (Math|Rotator|BreakRotator (Math|Rotator|FindLookatRotation (Transformation|GetWorldLocation (Variables|Default|GetSphere1)) (Transformation|GetActorLocation (Utilities|Array|Get(acopy) _outactors (Math|Random|RandomInteger (Utilities|Array|Length _outactors))))))) (+ (.Pitch (Math|Rotator|BreakRotator (Math|Rotator|FindLookatRotation (Transformation|GetWorldLocation (Variables|Default|GetSphere1)) (Transformation|GetActorLocation (Utilities|Array|Get(acopy) _outactors (Math|Random|RandomInteger (Utilities|Array|Length _outactors))))))) 4e+01) (.Yaw (Math|Rotator|BreakRotator (Math|Rotator|FindLookatRotation (Transformation|GetWorldLocation (Variables|Default|GetSphere1)) (Transformation|GetActorLocation (Utilities|Array|Get(acopy) _outactors (Math|Random|RandomInteger (Utilities|Array|Length _outactors))))))))) 2e+03) "None" true)
  (Utilities|FlowControl|Delay 1.0)
  (goto _label))

(event Custom|CE_MuzzleShot
  (bind _muzzle_flash (Variables|Default|GetMuzzle_Flash))
  (bind _muzzle_flash3 (Variables|Default|GetMuzzle_Flash3))
  (Timeline|Timeline PlayFromStart
    (:Finished
      (Rendering|SetVisibility (Variables|Default|GetMuzzle_Flash1) false false))
    (:NewTrack_1
      (Utilities|FlowControl|FlipFlop
        (:A
          (Rendering|SetVisibility _muzzle_flash3 true false)
          (Rendering|SetVisibility _muzzle_flash false false))
        (:B
          (Rendering|SetVisibility _muzzle_flash true false)
          (Rendering|SetVisibility _muzzle_flash3 false false))))))

(event EventBeginPlay
  (CallFunction|CECannonShot))

(fn ConstructionScript)