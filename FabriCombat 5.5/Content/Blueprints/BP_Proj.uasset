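; BP_Proj is an artillery shell projectile that deals area damage to enemy AI when it hits something.
; On hit, it spawns a nuke Niagara effect slightly above the impact, sends DamageMessage to every BP_EnemyAI overlapping its Sphere, then destroys itself.
; Each affected enemy's name is printed for debugging, and the damage call passes a zero impact point rather than the hit location.
; Two older Blueprint explosion spawns remain unconnected.
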(event OnComponentHit(ArtilleryShell)
  (params (HitComponent :type Primitive%20Component%20Object%20Reference) (OtherActor :type Actor%20Object%20Reference) (OtherComp :type Primitive%20Component%20Object%20Reference) (NormalImpulse :type Vector :default "0, 0, 0") (Hit :type Hit%20Result%20Structure%20%28by%20ref%29))
  (bind (_x _y _z) (Math|Vector|BreakVector (.location Hit)))
  (Niagara|SpawnSystematLocation "/Game/Niagara/NS_ACT_Nuke1.NS_ACT_Nuke1" (Math|Vector|MakeVector _x _y (+ _z 1e+02)))
  (for _array_element (Collision|GetOverlappingActors (Variables|Default|GetSphere) "/Game/Blueprints/BP_EnemyAI.BP_EnemyAI_C" :!class /Script/Engine.PrimitiveComponent)
    (Development|PrintString (Utilities|GetDisplayName _array_element))
    (Class|BPIInteract|Damage(Message) _array_element "0, 0, 0" false))
  (Actor|DestroyActor))

(fn ConstructionScript)