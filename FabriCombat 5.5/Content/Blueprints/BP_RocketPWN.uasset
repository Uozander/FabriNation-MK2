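; BP_RocketPWN is a cinematic homing missile that climbs after launch, then strikes a random BP_EnemyAI.
; Chained timelines lerp position and rotation through launch, approach and a final dive on the target's updated location.
; Its camera cuts to first-person for the chase and a side view after impact.
; It damages the target, plays a boom and self-destroys; if the target vanishes mid-approach, it drops to a fixed height and spawns an explosion.
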(event Custom|CE_Launch
  (params (Forward%20Vector :type Vector))
  (bind _firstpersontrans (Variables|Default|GetFirstPersonTrans))
  (bind _sidetrans (Variables|Default|GetSideTrans))
  (Variables|Default|SetForward%20Vector Forward%20Vector)
  (bind _newtrack_0 (Timeline|Timeline PlayFromStart)
    (:Update
      (Transformation|SetActorLocationAndRotation self (Math|Vector|Lerp(Vector) (Variables|Default|GetLock_Location) (+ (Variables|Default|GetLock_Location) (+ (* (Variables|Default|GetForward%20Vector) 4e+03) "0.000000,0.000000,4000.000000")) (Math|Float|Clamp(Float) (+ _newtrack_0 0.01))) (Math|Rotator|Lerp(Rotator) (Math|Rotator|MakeRotator (.roll (Math|Conversions|RotationFromXVector (Variables|Default|GetLock_Location))) (.pitch (Math|Conversions|RotationFromXVector (Variables|Default|GetLock_Location))) (+ (.yaw (Math|Conversions|RotationFromXVector (Variables|Default|GetLock_Location))) -9e+01)) (Math|Rotator|FindLookatRotation (Variables|Default|GetLock_Location) (+ (Variables|Default|GetLock_Location) (+ (* (Variables|Default|GetForward%20Vector) 4e+03) "0.000000,0.000000,4000.000000"))) (Math|Float|Clamp(Float) (* _newtrack_0 2.0)) true)))
    (:Finished
      (Utilities|FlowControl|Delay 0.1)
      (Variables|Default|SetLock_Location (Transformation|GetActorLocation))
      (bind _outactors (Actor|GetAllActorsOfClass "/Game/Blueprints/BP_EnemyAI.BP_EnemyAI_C"))
      (Utilities|IsValid (Utilities|Array|Get(acopy) _outactors (Math|Random|RandomInteger (Utilities|Array|Length _outactors))) :!label _label
        (:Is%20Valid
          (bind _output_get (Variables|Default|SetTarget (Utilities|Array|Get(acopy) _outactors (Math|Random|RandomInteger (Utilities|Array|Length _outactors)))))
          (Variables|Default|SetTarget_Location (Transformation|GetActorLocation _output_get))
          (Transformation|SetRelativeLocationAndRotation (Variables|Default|GetSphere) "0, 0, 0" "0.000000,90.000000,-20.000000" false false)
          (Transformation|SetRelativeLocationAndRotation (Variables|Default|GetCamera) (.location _firstpersontrans) (.rotation _firstpersontrans) false false)
          (bind _newtrack_0_2 (Timeline|Timeline_0 PlayFromStart)
            (:Update
              (Transformation|SetActorLocationAndRotation (Math|Vector|Lerp(Vector) (Variables|Default|GetLock_Location) (Variables|Default|GetTarget_Location) _newtrack_0_2) (Math|Rotator|Lerp(Rotator) (Math|Conversions|RotationFromXVector (Variables|Default|GetLock_Location)) (Math|Rotator|FindLookatRotation (Variables|Default|GetLock_Location) (Variables|Default|GetTarget_Location)) (Math|Float|Clamp(Float) (* _newtrack_0_2 2.0)) true)))
            (:Finished
              (Variables|Default|SetLock_Location (Transformation|GetWorldLocation (Variables|Default|GetStaticMesh)))
              (Utilities|IsValid (Variables|Default|GetTarget)
                (:Is%20Valid
                  (Variables|Default|SetTarget_Location (Transformation|GetActorLocation (Variables|Default|GetTarget)))
                  (Transformation|SetActorRotation (Math|Rotator|FindLookatRotation (Variables|Default|GetLock_Location) (Variables|Default|GetTarget_Location)))
                  (bind _newtrack_0_3 (Timeline|Timeline_1 PlayFromStart)
                    (:Update
                      (Transformation|SetActorLocation self (Math|Vector|Lerp(Vector) (Variables|Default|GetLock_Location) (Variables|Default|GetTarget_Location) _newtrack_0_3) false false))
                    (:Finished
                      (Utilities|IsValid (Variables|Default|GetTarget)
                        (:Is%20Valid
                          (Default|Damage (Variables|Default|GetTarget) "0, 0, 0" true 1))
                        (:Is%20Not%20Valid
                          _))
                      (CallFunction|CEBoom)
                      (Rendering|SetVisibility (Variables|Default|GetStaticMesh) false true)
                      (Transformation|SetRelativeLocationAndRotation (Variables|Default|GetSphere) "0, 0, 0" "0.000000,180.000000,-20.000000" false false)
                      (Transformation|SetRelativeLocationAndRotation (Variables|Default|GetCamera) (.location _sidetrans) (.rotation _sidetrans) false false)
                      (Transformation|SetWorldRotation (Variables|Default|GetSphere) "0.000000,0.000000,-20.000000" false false)
                      (Utilities|FlowControl|Delay 2.0)
                      (Actor|DestroyActor))))
                (:Is%20Not%20Valid
                  (Transformation|SetActorRotation (Math|Rotator|FindLookatRotation (Variables|Default|GetLock_Location) (Math|Vector|MakeVector (.X (Math|Vector|BreakVector (Variables|Default|GetLock_Location))) (.Y (Math|Vector|BreakVector (Variables|Default|GetLock_Location))) -5.5e+02)))
                  (bind _newtrack_0_4 (Timeline|Timeline_2 PlayFromStart)
                    (:Update
                      (Transformation|SetActorLocation self (Math|Vector|Lerp(Vector) (Variables|Default|GetLock_Location) (Math|Vector|MakeVector (.X (Math|Vector|BreakVector (Variables|Default|GetLock_Location))) (.Y (Math|Vector|BreakVector (Variables|Default|GetLock_Location))) -5.5e+02) _newtrack_0_4) false false))
                    (:Finished
                      (CallFunction|CEBoom)
                      (Rendering|SetVisibility (Variables|Default|GetStaticMesh) false true)
                      (Game|SpawnActorfromClass "/Game/StarterContent/Blueprints/Blueprint_Effect_Explosion.Blueprint_Effect_Explosion_C" (Math|Transform|MakeTransform (Transformation|GetWorldLocation (Variables|Default|GetStaticMesh)) "0, 0, 0" "1.000000,1.000000,1.000000") "Undefined" "MultiplyWithRoot" 0 0)
                      (Transformation|SetRelativeRotation (Variables|Default|GetSphere) "-40.000000,0.000000,0.000000" false false)
                      (Utilities|FlowControl|Delay 3.0)
                      (Actor|DestroyActor))))))))
        (:Is%20Not%20Valid
          (Utilities|FlowControl|Delay 0.01)
          (goto _label))))))

(event Custom|CE_Boom
  (Audio|PlaySoundatLocation "/Game/Sounds/explosion-47821.explosion-47821" (Transformation|GetActorLocation) "0, 0, 0" 0.1 1.0 0.4 0 0 0 0))

(event EventBeginPlay
  (Variables|Default|SetLock_Location (Transformation|GetActorLocation))
  (Components|Activation|Activate (Variables|Default|GetAudio) false))

(fn ConstructionScript)