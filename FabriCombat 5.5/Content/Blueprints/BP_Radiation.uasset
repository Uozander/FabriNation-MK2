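; BP_Radiation is a moving radiation hazard that poisons the enemy AI it touches.
; From BeginPlay, a Timeline slides the actor along world Y between its start position and a fixed offset, with a FlipFlop re-triggered on Finished to alternate direction endlessly.
; Every Tick, it polls overlapping BP_EnemyAI actors and calls PoisonMessage on each, so the effect repeats each frame while they overlap.
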(event EventBeginPlay
  (Variables|Default|SetDef_Loc (Transformation|GetActorLocation))
  (Utilities|FlowControl|FlipFlop :!label _label
    (:A
      (bind _newtrack_0 (Timeline|Timeline PlayFromStart)
        (:Update
          (Transformation|SetActorLocation (Math|Vector|MakeVector (.x (Variables|Default|GetDef_Loc)) (+ (.y (Variables|Default|GetDef_Loc)) (Math|Float|Lerp 0.0 -6.5e+03 _newtrack_0)) (.z (Variables|Default|GetDef_Loc))) false false))
        (:Finished
          (Utilities|FlowControl|Delay 0.02)
          (goto _label))))
    (:B
      (Timeline|Timeline ReverseFromEnd))))

(event EventTick
  (params (DeltaSeconds :type Float%20%28single-precision%29))
  (for _array_element (Collision|GetOverlappingActors "/Game/Blueprints/BP_EnemyAI.BP_EnemyAI_C" :!class /Script/Engine.Actor)
    (Class|BPIInteract|Poison(Message) _array_element)))

(fn ConstructionScript)