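; Enemy spawner Blueprint that creates BP_EnemyAI pawns running BT_AI at the location of its Sphere component.
; On BeginPlay it spawns one enemy at a fixed interval for as long as Active stays true, using a looped Delay.
; The CE_Wave event separately spawns a burst of Count enemies, counting down with a very short Delay between spawns.
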(event Custom|CE_Wave
  (params (Count :type Integer))
  (Variables|Default|SetCount Count)
  (if (> (Variables|Default|GetCount) 0) :!label _label
    (AI|SpawnAIFromClass "/Game/Blueprints/BP_EnemyAI.BP_EnemyAI_C" "/Game/AI/BT_AI.BT_AI" (Transformation|GetWorldLocation (Variables|Default|GetSphere)) "0, 0, 0" false 0)
    (Variables|Default|SetCount (- (Variables|Default|GetCount) 1))
    (Utilities|FlowControl|Delay 0.01)
    (goto _label)))

(event EventBeginPlay
  (if (Variables|Default|GetActive) :!label _label
    (AI|SpawnAIFromClass "/Game/Blueprints/BP_EnemyAI.BP_EnemyAI_C" "/Game/AI/BT_AI.BT_AI" (Transformation|GetWorldLocation (Variables|Default|GetSphere)) "0, 0, 0" false 0)
    (Utilities|FlowControl|Delay 1e+01)
    (goto _label)))

(fn ConstructionScript)