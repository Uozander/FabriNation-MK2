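; BP_SPAWN_Citizen is a spawn point that creates an AI BP_Citizen2 at its Sphere component's location on BeginPlay when Active is set.
; It copies its Kinetic, Missile and Energy UP variables (tiers 1, 2, 3a and 3b) onto the new citizen.
; A one-second delay leading back into the spawn is left unconnected, so only one spawn is attempted.
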(event EventBeginPlay
  (if (Variables|Default|GetActive)
    (bind _returnvalue (AI|SpawnAIFromClass "/Game/BP_Citizen2.BP_Citizen2_C" 0 (Transformation|GetWorldLocation (Variables|Default|GetSphere)) "0, 0, 0" false 0))
    (bind _asbp_citizen_2 (Utilities|Casting|CastToBP_Citizen2 _returnvalue))
    (Variables|/Game/BP_Citizen2.BP_Citizen2_C|SetKineticUP1 _asbp_citizen_2 (Variables|Default|GetKinetic%20UP1))
    (Variables|/Game/BP_Citizen2.BP_Citizen2_C|SetMissileUP1 _asbp_citizen_2 (Variables|Default|GetMissile%20UP1))
    (Variables|/Game/BP_Citizen2.BP_Citizen2_C|SetEnergyUP1 _asbp_citizen_2 (Variables|Default|GetEnergy%20UP1))
    (Variables|/Game/BP_Citizen2.BP_Citizen2_C|SetKineticUP2 _asbp_citizen_2 (Variables|Default|GetKinetic%20UP2))
    (Variables|/Game/BP_Citizen2.BP_Citizen2_C|SetMissileUP2 _asbp_citizen_2 (Variables|Default|GetMissile%20UP2))
    (Variables|/Game/BP_Citizen2.BP_Citizen2_C|SetEnergyUP2 _asbp_citizen_2 (Variables|Default|GetEnergy%20UP2))
    (Variables|/Game/BP_Citizen2.BP_Citizen2_C|SetKineticUP3a _asbp_citizen_2 (Variables|Default|GetKinetic%20UP3a))
    (Variables|/Game/BP_Citizen2.BP_Citizen2_C|SetMissileUP3a _asbp_citizen_2 (Variables|Default|GetMissile%20UP3a))
    (Variables|/Game/BP_Citizen2.BP_Citizen2_C|SetEnergyUP3a _asbp_citizen_2 (Variables|Default|GetEnergy%20UP3a))
    (Variables|/Game/BP_Citizen2.BP_Citizen2_C|SetKineticUP3b%20 _asbp_citizen_2 (Variables|Default|GetKinetic%20UP3b))
    (Variables|/Game/BP_Citizen2.BP_Citizen2_C|SetMissileUP3b _asbp_citizen_2 (Variables|Default|GetMissile%20UP3b))
    (Variables|/Game/BP_Citizen2.BP_Citizen2_C|SetEnergyUP3b _asbp_citizen_2 (Variables|Default|GetEnergy%20UP3b))))

(fn ConstructionScript)