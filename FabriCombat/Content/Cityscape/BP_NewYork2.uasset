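; BP_NewYork2 is a cityscape actor that disappears in a Niagara effect when a BP_Industry actor overlaps it.
; The first Box overlap by that exact class activates Niagara, toggles the static mesh's visibility, then destroys the actor five seconds later.
; A CE_Dust event can trigger the effect separately, while an alternate delayed sequence and an NS_DUST spawn are left unwired.
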(event OnComponentBeginOverlap(Box)
  (params (OverlappedComponent :type Primitive%20Component%20Object%20Reference) (OtherActor :type Actor%20Object%20Reference) (OtherComp :type Primitive%20Component%20Object%20Reference) (OtherBodyIndex :type Integer) (bFromSweep :type Boolean) (SweepResult :type Hit%20Result%20Structure%20%28by%20ref%29))
  (if (== (Utilities|GetClass OtherActor) "/Game/Buildings/BP_Industry.BP_Industry_C")
    (Utilities|FlowControl|DoOnce false
      (:Completed
        (Components|Activation|Activate (Variables|Default|GetNiagara) false)
        (Rendering|ToggleVisibility (Variables|Default|GetStaticMesh) false)
        (Utilities|FlowControl|Delay 5.0)
        (Actor|DestroyActor)))))

(event Custom|CE_Dust
  (Components|Activation|Activate (Variables|Default|GetNiagara) false))

(event EventBeginPlay)

(event Collision|EventActorBeginOverlap
  (params (OtherActor :type Actor%20Object%20Reference)))

(event EventTick
  (params (DeltaSeconds :type Float%20%28single-precision%29)))

(event Input|KeyboardEvents|G
  (params (Key :type Key%20Structure)))

(fn ConstructionScript)