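; Necrotitanium processing building that turns delivered ore into Steel, dispatching a truck once 40 is stocked.
; BeginPlay removes it if overlapping a non-transparent industry, drains player Wealth every second, and traces for an industry neighbour to show tubes and cut that upkeep.
; Work events consume ore and toggle smoke, scaled by a multiplier that upgrade events set.
; Citizen events count workers and trace random directions to spawn or tier up housing.
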(event Custom|CE_HomeSpawn
  (params (Citizen :type Actor%20Object%20Reference))
  (Variables|Default|SetCitizen Citizen)
  (switch int (Math|Random|RandomInteger 4)
    (:0
      (CallFunction|SpawnHome (Variables|Default|GetNorth) (Variables|Default|GetCitizen)))
    (:1
      (CallFunction|SpawnHome (Variables|Default|GetSouth) (Variables|Default|GetCitizen)))
    (:2
      (CallFunction|SpawnHome (Variables|Default|GetWest) (Variables|Default|GetCitizen)))
    (:3
      (CallFunction|SpawnHome (Variables|Default|GetEast) (Variables|Default|GetCitizen)))))

(event Custom|CE_Work
  (bind _necrotitanium_cost (Variables|Default|GetNecrotitanium%20Cost))
  (bind _upgrade_multiplier (Variables|Default|GetUpgrade_Multiplier))
  (bind _returnvalue (* _necrotitanium_cost _upgrade_multiplier))
  (if (>= (Variables|Default|GetNecrotitanium%20Ore) _returnvalue)
    (Math|Float|IncrementFloat (Variables|Default|GetSuccess)
      (:%20%20
        (Variables|Default|SetSteel_Track (+ (Variables|Default|GetSteel_Track) 2))
        (Variables|Default|SetNecrotitanium%20Ore (Math|Integer|Clamp(Integer) (- (Variables|Default|GetNecrotitanium%20Ore) _returnvalue) 0 1000))
        (Variables|Default|SetGoods (Utilities|Struct|MakeSTCT_Resource (+ (.ore_amount (Variables|Default|GetGoods)) (* (Variables|Default|GetSteel%20Output) (Variables|Default|GetUpgrade_Multiplier))) "Steel" 0))
        (Components|Activation|Activate (Variables|Default|GetP_SmokestackFog) false)
        (Rendering|Components|TextRender|SetText (Variables|Default|GetTextRender) (Utilities|Text|ToText(Integer) (Variables|Default|GetNecrotitanium%20Ore)))
        (Rendering|SetVisibility (Variables|Default|GetP_SmokestackFog) true false)
        (if (>= (.ore_amount (Variables|Default|GetGoods)) 40)
          (CallFunction|CETruck))))
    (else
      (Math|Float|IncrementFloat (Variables|Default|GetFail)
        (:%20%20
          (Components|Activation|Deactivate (Variables|Default|GetP_SmokestackFog2))
          (Rendering|SetVisibility (Variables|Default|GetP_SmokestackFog) false false))))))

(event Custom|CE_WorkerUP
  (Variables|Default|SetWorkers (+ (Variables|Default|GetWorkers) 1))
  (bind _asbp_top_down_controller (Utilities|Casting|CastToBP_TopDownController (Game|GetPlayerController 0)))
  (Variables|/Game/TopDown/Blueprints/BP_TopDownController.BP_TopDownController_C|SetCitizens _asbp_top_down_controller (+ (Variables|/Game/TopDown/Blueprints/BP_TopDownController.BP_TopDownController_C|GetCitizens _asbp_top_down_controller) 1.0)))

(event Custom|CE_Deliver
  (params (Delivery :type STCT%20Resource%20Structure))
  (switch int (.ore_number Delivery)
    (:1
      (Variables|Default|SetNecrotitanium%20Ore (Math|Integer|Clamp(Integer) (+ (.ore_amount Delivery) (Variables|Default|GetNecrotitanium%20Ore)) 0 1000)))
    (:2
      (bind _output_get (Variables|Default|SetNecrotitanium (+ (.ore_amount Delivery) (Variables|Default|GetNecrotitanium))))
      (Rendering|Components|TextRender|SetText (Variables|Default|GetTextRender) (Utilities|Text|ToText(Integer) _output_get)))))

(event Custom|CE_Truck
  (bind _returnvalue (Game|SpawnActorfromClass "/Game/Units/BP_Truck.BP_Truck_C" (Transformation|GetActorTransform) "Undefined" "MultiplyWithRoot" 0 0))
  (Default|CEDeliver _returnvalue (Variables|Default|GetGoods))
  (Variables|Default|SetGoods (Utilities|Struct|MakeSTCT_Resource 0 "Steel" 0)))

(event Custom|CE_Upgrade_2
  (Rendering|SetVisibility (Variables|Default|GetEdge7) true false)
  (Variables|Default|SetUpgrade_Multiplier 2.5)
  (Variables|Default|SetUpgrade2? true))

(event Custom|CE_Upgrade_1
  (Rendering|SetVisibility (Variables|Default|GetCorner1) true false)
  (Variables|Default|SetUpgrade_Multiplier 4.0)
  (Variables|Default|SetUpgrade1? true))

(event Custom|CE_Demo
  (Collision|SetCollisionEnabled (Variables|Default|GetCube7) "NoCollision")
  (Game|SpawnActorfromClass "/Game/Buildings/BP_DEMO_Ind.BP_DEMO_Ind_C" (Transformation|GetActorTransform self) "Undefined" "MultiplyWithRoot" 0 0)
  (Actor|DestroyActor))

(event Custom|CE_Upgrade_3
  (Rendering|SetVisibility (Variables|Default|GetTop2) true false)
  (Variables|Default|SetUpgrade_Multiplier 1.5)
  (Variables|Default|SetUpgrade3? true))

(event EventBeginPlay
  (bind _overlappingactors (Collision|GetOverlappingActors "/Game/Buildings/BP_Industry.BP_Industry_C" :!class /Script/Engine.Actor))
  (Variables|Default|SetIndustry%20Name (Utilities|SetName))
  (Utilities|FlowControl|Sequence
    (:then_0
      (Utilities|FlowControl|Delay 0.1)
      (if (not (Utilities|Array|IsEmpty _overlappingactors))
        (Utilities|IsValid (Variables|Default|GetBox)
          (:Is%20Valid
            (for _array_element _overlappingactors
              (if (== (Utilities|GetClass _array_element) "/Game/Buildings/BP_Industry.BP_Industry_C")
                (bind _asbp_industry (Utilities|Casting|CastToBP_Industry _array_element))
                (Utilities|IsValid (Variables|/Game/Buildings/BP_Industry.BP_Industry_C|GetStructure _asbp_industry)
                  (:Is%20Valid
                    (if (not (== (Rendering|Material|GetMaterial (Variables|/Game/Buildings/BP_Industry.BP_Industry_C|GetStructure _asbp_industry) 0) "/Game/Materials/MAT_Trans.MAT_Trans"))
                      (Actor|DestroyActor))))))))))
    (:then_1
      (bind _asbp_top_down_controller (Utilities|Casting|CastToBP_TopDownController (Game|GetPlayerController 0)))
      (Variables|Default|SetAs%20BP%20Top%20Down%20Controller _asbp_top_down_controller)
      (Utilities|FlowControl|Delay 1.0 :!label _label)
      (Variables|/Game/TopDown/Blueprints/BP_TopDownController.BP_TopDownController_C|SetWealth (Variables|Default|GetAs%20BP%20Top%20Down%20Controller) (- (Variables|/Game/TopDown/Blueprints/BP_TopDownController.BP_TopDownController_C|GetWealth (Variables|Default|GetAs%20BP%20Top%20Down%20Controller)) (Variables|Default|GetCost)))
      (goto _label))
    (:then_2
      (Utilities|FlowControl|Delay 0.2)
      (bind _hit (CallFunction|CheckAdjacent (Variables|Default|GetNorth)))
      (if _hit
        (Rendering|SetVisibility (Variables|Default|GetNorthTube2) true false)
        (Variables|Default|SetCost (- (Variables|Default|GetCost) 8.0) :!label _label_2)
        (else
          (bind _hit_2 (CallFunction|CheckAdjacent (Variables|Default|GetSouth)))
          (if _hit_2
            (Rendering|SetVisibility (Variables|Default|GetSouthTube4) true false)
            (goto _label_2)
            (else
              (bind _hit_3 (CallFunction|CheckAdjacent (Variables|Default|GetEast)))
              (if _hit_3
                (Rendering|SetVisibility (Variables|Default|GetEastTube7) true false)
                (goto _label_2)
                (else
                  (bind _hit_4 (CallFunction|CheckAdjacent (Variables|Default|GetWest)))
                  (if _hit_4
                    (Rendering|SetVisibility (Variables|Default|GetWestTube9) true false)
                    (goto _label_2)))))))))))

(fn ConstructionScript)

(fn SpawnHome
  (params (Direction :type Vector) (Citizen :type Actor%20Object%20Reference))
  (bind _structure (Variables|Default|GetStructure))
  (bind _returnvalue (Transformation|GetWorldLocation _structure))
  (bind _returnvalue_2 (+ _returnvalue Direction))
  (bind _returnvalue_3 (- _returnvalue_2 "0.000000,0.000000,50.000000"))
  (bind (_outhit _returnvalue_4) (Collision|LineTraceByChannel (+ _returnvalue "0.000000,0.000000,50.000000") _returnvalue_2 "TraceTypeQuery1" false 0 "None"))
  (if _returnvalue_4
    (if (== (Utilities|GetClass (.HitActor (Collision|BreakHitResult _outhit))) "/Game/Buildings/BP_Residential.BP_Residential_C")
      (bind _asbp_residential (Utilities|Casting|CastToBP_Residential (.HitActor (Collision|BreakHitResult _outhit))))
      (if (>= (Variables|/Game/Buildings/BP_Residential.BP_Residential_C|GetLevel _asbp_residential) (Variables|/Game/Buildings/BP_Residential.BP_Residential_C|GetMax%20Tier _asbp_residential))
        (Default|CEHomeSpawn _asbp_residential Citizen)
        (else
          (Default|CETierUp _asbp_residential Citizen)))
      (else
        (Actor|DestroyActor Citizen)))
    (else
      (Game|SpawnActorfromClass "/Game/Buildings/BP_Residential.BP_Residential_C" (Math|Transform|MakeTransform _returnvalue_3 "0, 0, 0" "1.000000,1.000000,1.000000") "Undefined" "MultiplyWithRoot" 0 0)
      (bind _asbp_citizen (Utilities|Casting|CastToBP_Citizen Citizen))
      (Variables|/Game/Units/BP_Citizen.BP_Citizen_C|SetHome%20Location _asbp_citizen _returnvalue_3))))

(fn CheckAdjacent
  (params (Direction :type Vector))
  (bind _structure (Variables|Default|GetStructure))
  (bind _returnvalue (Transformation|GetWorldLocation _structure))
  (bind _outhit (Collision|LineTraceByChannel (+ _returnvalue "0.000000,0.000000,50.000000") (+ _returnvalue Direction) "TraceTypeQuery1" false 0 "None"))
  (return (== (Utilities|GetClass (.HitActor (Collision|BreakHitResult _outhit))) "/Game/Buildings/BP_Industry.BP_Industry_C")))