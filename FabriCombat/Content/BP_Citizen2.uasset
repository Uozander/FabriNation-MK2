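; AI citizen that wanders the navmesh, fights perceived tagged targets and levels up at shops.
; AI Perception locks a target, then it closes to range, aims, line-traces with random spread, fires blaster bursts and reloads, using BP_Nobody as a null-target sentinel.
; Damaging hits earn XP; each level sends it to a random shop for a medical, weapon or armor upgrade.
; Incoming damage is divided by armor, and death triggers ragdoll before destruction.
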(event OnTargetPerceptionUpdated(AIPerception)
  (params (Actor :type Actor%20Object%20Reference) (Stimulus :type AI%20Stimulus%20Structure))
  (if (Variables|Default|GetLocked)
    (CallFunction|CEFindTarget)
    (elif (not (Variables|AI|Getseeking%20upgrade))
      (if (Actor|ActorHasTag Actor (Variables|AI|GetTag))
        (Utilities|IsValid Actor
          (:Is%20Valid
            (Variables|AI|SetTarget Actor)
            (Variables|Default|SetLocked true)
            (Variables|AI|SetSeePlayer true)
            (CallFunction|CEFollow)))
        (else
          (CallFunction|CESearch))))))

(event Custom|CE_Swing
  ;[1 0.4635 0] DEP
  (bind _newtrack_2 (Timeline|Timeline_0 PlayFromStart)
    (:Update
      (Transformation|SetRelativeRotation (Variables|Default|Getrr) (Math|Rotator|MakeRotator 0.0 (Math|Float|Lerp 0.0 -1.1e+02 _newtrack_2) 0.0) false false))
    (:Finished
      (Transformation|SetRelativeRotation (Variables|Default|Getrr) (Math|Rotator|MakeRotator 0.0 0.0 0.0) false false))))

(event Custom|CE_Search
  (bind _self self)
  (bind _returnvalue (Transformation|GetActorLocation _self))
  (bind (_randomlocation _returnvalue_2) (AI|Navigation|GetRandomReachablePointinRadius _returnvalue 2e+03 0 0))
  (if (not (Variables|AI|GetSeePlayer))
    (Variables|AI|SetSearching true)
    (if _returnvalue_2
      (AI|AIMoveTo self _randomlocation 0 1.5e+02 false
        (:OnSuccess
          _)
        (:OnFail
          _))
      (Variables|AI|SetSearching false)
      (Variables|AI|SetSeePlayer false)
      (CallFunction|CESearch))))

(event Custom|CE_Widget
  (bind _returnvalue (AddComponent|AddWidgetComponent false (Math|Transform|MakeTransform (Variables|AI|GetRelative%20Transform%20Location) "0, 0, 0" "0.100000,0.100000,0.100000")))
  (bind _returnvalue_2 (Game|ConstructObjectfromClass _returnvalue "/Game/WDG_Level.WDG_Level_C"))
  (Variables|Other|SetWIDGET_ _returnvalue_2)
  (UserInterface|SetWidget (Variables|Default|GetWidget_Space) _returnvalue_2))

(event Custom|CE_Blaster
  (bind _target (Variables|AI|GetTarget))
  (bind _arrow1 (Variables|Default|GetArrow1))
  ;[1 1 1] Blaster
  (if (not (== (Utilities|GetClass _target) "/Game/BP_Nobody.BP_Nobody_C"))
    (Utilities|IsValid _target
      (:Is%20Valid
        (bind _output_get (Variables|AI|SetBlaster_Target _target))
        (if (Utilities|IsValid _output_get)
          (if (not (Utilities|Operators|EqualEqual :A (.Location (Math|Transform|BreakTransform (.Transform (Utilities|BlasterSpread _output_get _arrow1 (Transformation|GetWorldLocation _arrow1) (Transformation|GetActorLocation _output_get) (Transformation|GetWorldScale _arrow1)))))))
            (bind _output_get_2 (Variables|Default|SetTransform (.Transform (Utilities|BlasterSpread _output_get _arrow1 (Transformation|GetWorldLocation _arrow1) (Transformation|GetActorLocation _output_get) (Transformation|GetWorldScale _arrow1)))))
            (Variables|Default|SetImpulse (* (Math|Rotator|GetRotationXVector (.Rotator (Utilities|BlasterSpread _output_get _arrow1 (Transformation|GetWorldLocation _arrow1) (Transformation|GetActorLocation _output_get) (Transformation|GetWorldScale _arrow1)))) 1.5e+04))
            (bind _returnvalue (Game|SpawnActorfromClass "/Game/BP_Blaster1.BP_Blaster1_C" _output_get_2 "AdjustIfPossibleButAlwaysSpawn" "MultiplyWithRoot" 0 0))
            (Audio|SpawnSoundatLocation "/Game/META_Blaster.META_Blaster" (.location (Variables|Default|GetTransform)) "0, 0, 0" 1.0 1.0 0.0 0 0)
            (Physics|AddImpulse (Variables|/Game/BP_Blaster1.BP_Blaster1_C|GetSphere _returnvalue) (Variables|Default|GetImpulse) "None" true)
            (Utilities|FlowControl|Delay 0.1)
            (bind _returnvalue_2 (Game|SpawnActorfromClass "/Game/BP_Blaster1.BP_Blaster1_C" (Variables|Default|GetTransform) "AdjustIfPossibleButAlwaysSpawn" "MultiplyWithRoot" 0 0))
            (Audio|SpawnSoundatLocation "/Game/META_Blaster.META_Blaster" (.location (Variables|Default|GetTransform)) "0, 0, 0" 1.0 1.0 0.0 0 0)
            (Physics|AddImpulse (Variables|/Game/BP_Blaster1.BP_Blaster1_C|GetSphere _returnvalue_2) (Variables|Default|GetImpulse) "None" true)
            (Utilities|FlowControl|Delay 0.1)
            (bind _returnvalue_3 (Game|SpawnActorfromClass "/Game/BP_Blaster1.BP_Blaster1_C" (Variables|Default|GetTransform) "AdjustIfPossibleButAlwaysSpawn" "MultiplyWithRoot" 0 0))
            (Audio|SpawnSoundatLocation "/Game/META_Blaster.META_Blaster" (.location (Variables|Default|GetTransform)) "0, 0, 0" 1.0 1.0 0.0 0 0)
            (Physics|AddImpulse (Variables|/Game/BP_Blaster1.BP_Blaster1_C|GetSphere _returnvalue_3) (Variables|Default|GetImpulse) "None" true))))
      (:Is%20Not%20Valid
        (Development|PrintString "INVALID")))))

(event Custom|CE_Print
  ;[1 0.9008 0] Print PERCEIVED actors
)

(event Custom|CE_Attack
  (if (Variables|AI|GetReloading)
    (CallFunction|CEReload)
    (else
      (Variables|AI|SetReloading true)
      (Rendering|Material|SetMaterial (Variables|Character|GetMesh) 0 "/Game/MAT_Black.MAT_Black")
      (Utilities|FlowControl|Delay (Variables|Stats|GetAim%20Delay))
      (Utilities|IsValid (Variables|AI|GetTarget)
        (:Is%20Valid
          (if (== (Utilities|GetClass (Variables|AI|GetTarget)) "/Game/BP_Nobody.BP_Nobody_C")
            (CallFunction|CEFindTarget :!label _label)
            (elif (Utilities|Operators|EqualEqual :A (Transformation|GetActorLocation (Variables|AI|GetTarget)))
              (goto _label)
              (else
                (bind _outhit (Collision|LineTraceForObjects (Transformation|GetActorLocation self) (Math|Vector|MakeVector (Utilities|Spread (.x (Transformation|GetActorLocation (Variables|AI|GetTarget)))) (Utilities|Spread (.y (Transformation|GetActorLocation (Variables|AI|GetTarget)))) (Utilities|Spread (.z (Transformation|GetActorLocation (Variables|AI|GetTarget))))) (Variables|AI|GetObject%20Types_0) false 0 "ForOneFrame"))
                (if (.bblockinghit _outhit)
                  (CallFunction|CEBlaster)
                  (Utilities|FlowControl|Delay 0.2)
                  (Utilities|IsValid (.hitactor _outhit)
                    (:Is%20Valid
                      (Class|BPIInteract|Damage(Message) (.hitactor _outhit) (.impactpoint _outhit))
                      (Variables|AI|SetTarget (Variables|Default|GetNOBODY))
                      (Variables|Stats|SetXP (+ (Variables|Stats|GetXP) 1.0))
                      (if (>= (Variables|Stats|GetXP) (Variables|Stats|GetLevel%20req))
                        (Rendering|Material|SetMaterial (Variables|Character|GetMesh) 0 "/Game/MAT_Green.MAT_Green")
                        (Variables|AI|SetReloading false)
                        (CallFunction|CELevelUP)
                        (else
                          ;[0 0.6062 1] Reload
                          (Utilities|FlowControl|Delay (Variables|Stats|GetReload%20Time) :!label _label_2)
                          (Rendering|Material|SetMaterial (Variables|Character|GetMesh) 0 "/Game/Characters/Mannequins/Materials/Instances/Quinn/MI_Quinn_01.MI_Quinn_01")
                          (Variables|AI|SetReloading false)
                          ;[1 1 1] Find nearby target
                          (bind _array_element (Utilities|Array|ForEachLoopwithBreak (Class|AIPerceptionComponent|GetCurrentlyPerceivedActors (Variables|Default|GetAIPerception)) :!label _label_3)
                            (:LoopBody
                              (if (== (Utilities|GetClass _array_element) "/Game/BP_EnemyAI.BP_EnemyAI_C")
                                (Variables|AI|SetTarget _array_element)
                                (Utilities|FlowControl|Sequence
                                  (:then_0
                                    (CallFunction|CEAttack))
                                  (:then_1
                                    (goto _label_3 Break)))))
                            (:Completed
                              (CallFunction|CESearch)
                              (Variables|Default|SetLocked false))))))
                    (:Is%20Not%20Valid
                      (goto _label_2)))
                  (else
                    (CallFunction|CEBlaster)
                    (Utilities|FlowControl|Delay 0.2)
                    (goto _label_2)))))))
        (:Is%20Not%20Valid
          (goto _label))))))

(event Custom|CE_Splash
  (Niagara|SpawnSystematLocation "/Game/CE_StickImpact.CE_StickImpact" (Transformation|GetWorldLocation (Variables|Character|GetMesh))))

(event Custom|CE_Find%20Target
  ;[1 1 1] Find nearby target
  (Class|AIPerceptionComponent|ForgetAll (Variables|Default|GetAIPerception))
  (bind _array_element (Utilities|Array|ForEachLoopwithBreak (Class|AIPerceptionComponent|GetCurrentlyPerceivedActors (Variables|Default|GetAIPerception)) :!label _label)
    (:LoopBody
      (if (== (Utilities|GetClass _array_element) "/Game/BP_EnemyAI.BP_EnemyAI_C")
        (Variables|AI|SetTarget _array_element)
        (Utilities|FlowControl|Sequence
          (:then_0
            (CallFunction|CEAttack))
          (:then_1
            (goto _label Break)))))
    (:Completed
      (CallFunction|CESearch)
      (Variables|Default|SetLocked false))))

(event Custom|CE_Reload
  ;[0 0.6062 1] Reload
  (Utilities|FlowControl|Delay (Variables|Stats|GetReload%20Time))
  (Rendering|Material|SetMaterial (Variables|Character|GetMesh) 0 "/Game/Characters/Mannequins/Materials/Instances/Quinn/MI_Quinn_01.MI_Quinn_01")
  (Variables|AI|SetReloading false)
  ;[1 1 1] Find nearby target
  (bind _array_element (Utilities|Array|ForEachLoopwithBreak (Class|AIPerceptionComponent|GetCurrentlyPerceivedActors (Variables|Default|GetAIPerception)) :!label _label)
    (:LoopBody
      (if (== (Utilities|GetClass _array_element) "/Game/BP_EnemyAI.BP_EnemyAI_C")
        (Variables|AI|SetTarget _array_element)
        (Utilities|FlowControl|Sequence
          (:then_0
            (CallFunction|CEAttack))
          (:then_1
            (goto _label Break)))))
    (:Completed
      (CallFunction|CESearch)
      (Variables|Default|SetLocked false))))

(event Custom|CE_Windup
  ;[1 0.4635 0] DEP
  (bind _newtrack_2 (Timeline|Timeline PlayFromStart)
    (:Update
      (Variables|Deprecated|SetWindup _newtrack_2)
      (Transformation|SetRelativeRotation (Variables|Default|Getrr) (Math|Rotator|MakeRotator 0.0 (Math|Float|Lerp 0.0 55.0 _newtrack_2) 0.0) false false))))

(event Custom|CE_Follow
  (AI|AIMoveTo self (Transformation|GetActorLocation (Variables|AI|GetTarget)) 0 (- (Variables|Stats|GetRange) 5e+01) false :!label _label
    (:OnSuccess
      (Variables|AI|SetSeePlayer false)
      (Utilities|IsValid (Variables|AI|GetTarget)
        (:Is%20Valid
          (if (> (Transformation|GetDistanceTo (Variables|AI|GetTarget) self) (Variables|Stats|GetRange))
            (goto _label)
            (else
              (Components|Movement|StopMovementImmediately (Variables|Character|GetCharacterMovement))
              (if (Variables|AI|GetReloading)
                (CallFunction|CEReload)
                (else
                  (Variables|AI|SetReloading true)
                  (Rendering|Material|SetMaterial (Variables|Character|GetMesh) 0 "/Game/MAT_Black.MAT_Black")
                  (Utilities|FlowControl|Delay (Variables|Stats|GetAim%20Delay))
                  (Utilities|IsValid (Variables|AI|GetTarget)
                    (:Is%20Valid
                      (if (== (Utilities|GetClass (Variables|AI|GetTarget)) "/Game/BP_Nobody.BP_Nobody_C")
                        (CallFunction|CEFindTarget :!label _label_2)
                        (elif (Utilities|Operators|EqualEqual :A (Transformation|GetActorLocation (Variables|AI|GetTarget)))
                          (goto _label_2)
                          (else
                            (bind _outhit (Collision|LineTraceForObjects (Transformation|GetActorLocation self) (Math|Vector|MakeVector (Utilities|Spread (.x (Transformation|GetActorLocation (Variables|AI|GetTarget)))) (Utilities|Spread (.y (Transformation|GetActorLocation (Variables|AI|GetTarget)))) (Utilities|Spread (.z (Transformation|GetActorLocation (Variables|AI|GetTarget))))) (Variables|AI|GetObject%20Types_0) false 0 "ForOneFrame"))
                            (if (.bblockinghit _outhit)
                              (CallFunction|CEBlaster)
                              (Utilities|FlowControl|Delay 0.2)
                              (Utilities|IsValid (.hitactor _outhit)
                                (:Is%20Valid
                                  (Class|BPIInteract|Damage(Message) (.hitactor _outhit) (.impactpoint _outhit))
                                  (Variables|AI|SetTarget (Variables|Default|GetNOBODY))
                                  (Variables|Stats|SetXP (+ (Variables|Stats|GetXP) 1.0))
                                  (if (>= (Variables|Stats|GetXP) (Variables|Stats|GetLevel%20req))
                                    (Rendering|Material|SetMaterial (Variables|Character|GetMesh) 0 "/Game/MAT_Green.MAT_Green")
                                    (Variables|AI|SetReloading false)
                                    (CallFunction|CELevelUP)
                                    (else
                                      ;[0 0.6062 1] Reload
                                      (Utilities|FlowControl|Delay (Variables|Stats|GetReload%20Time) :!label _label_3)
                                      (Rendering|Material|SetMaterial (Variables|Character|GetMesh) 0 "/Game/Characters/Mannequins/Materials/Instances/Quinn/MI_Quinn_01.MI_Quinn_01")
                                      (Variables|AI|SetReloading false)
                                      ;[1 1 1] Find nearby target
                                      (bind _array_element (Utilities|Array|ForEachLoopwithBreak (Class|AIPerceptionComponent|GetCurrentlyPerceivedActors (Variables|Default|GetAIPerception)) :!label _label_4)
                                        (:LoopBody
                                          (if (== (Utilities|GetClass _array_element) "/Game/BP_EnemyAI.BP_EnemyAI_C")
                                            (Variables|AI|SetTarget _array_element)
                                            (Utilities|FlowControl|Sequence
                                              (:then_0
                                                (CallFunction|CEAttack))
                                              (:then_1
                                                (goto _label_4 Break)))))
                                        (:Completed
                                          (CallFunction|CESearch)
                                          (Variables|Default|SetLocked false))))))
                                (:Is%20Not%20Valid
                                  (goto _label_3)))
                              (else
                                (CallFunction|CEBlaster)
                                (Utilities|FlowControl|Delay 0.2)
                                (goto _label_3)))))))
                    (:Is%20Not%20Valid
                      (goto _label_2))))))))
        (:Is%20Not%20Valid
          (CallFunction|CESearch))))
    (:OnFail
      (CallFunction|CESearch))))

(event Custom|CE_Level_UP
  ;[1 1 1] LEVEL UP
  (Variables|Stats|SetLevel%20req (* (Variables|Stats|GetLevel%20req) 2.5))
  (Variables|AI|Setseeking%20upgrade true)
  (bind _output_get (Variables|Stats|SetLevel (+ (Variables|Stats|GetLevel) 1)))
  (Variables|/Script/UMG.TextBlock|SetText (Variables|/Game/WDG_Level.WDG_Level_C|GetTextBlock_0 (Variables|Other|GetWIDGET_)) (Utilities|Text|ToText(Integer) _output_get))
  (bind _outactors (Actor|GetAllActorsOfClass "/Game/BP_Shop.BP_Shop_C"))
  (bind _output_get_2 (Variables|AI|SetShop (Utilities|Array|Get(acopy) _outactors (Math|Random|RandomInteger (Utilities|Array|Length _outactors)))))
  (AI|AIMoveTo self (.RandomLocation (AI|Navigation|GetRandomReachablePointinRadius (Transformation|GetActorLocation _output_get_2) 3e+01 0 0)) 0 3e+02 false
    (:OnSuccess
      (CallFunction|CEUpgrade))
    (:OnFail
      (Variables|AI|Setseeking%20upgrade false)
      (Rendering|Material|SetMaterial (Variables|Character|GetMesh) 0 "/Game/Characters/Mannequins/Materials/Instances/Quinn/MI_Quinn_01.MI_Quinn_01")
      (CallFunction|CESearch))))

(event Custom|CE_UPdate
  ;[1 0.8313 0] Widget pointing
  (CallFunction|CEWidget))

(event Custom|CE_Upgrade
  ;[1 1 1] LEVEL UP
  (switch int (Variables|/Game/BP_Shop.BP_Shop_C|GetShop%20Type (stale Custom|CE_Level_UP _output_get_2))
    (:0
      (CallFunction|CEMedical))
    (:1
      (CallFunction|CEWeapons))
    (:2
      (CallFunction|CEArmor)))
  (Variables|AI|Setseeking%20upgrade false)
  (Rendering|Material|SetMaterial (Variables|Character|GetMesh) 0 "/Game/Characters/Mannequins/Materials/Instances/Quinn/MI_Quinn_01.MI_Quinn_01")
  (CallFunction|CESearch))

(event Custom|CE_Medical
  ;[1 1 1] LEVEL UP
  ;;[1 1 1] Upgrades
  (Variables|Stats|SetHP (+ (Variables|Stats|GetHP) 1.0)))

(event Custom|CE_Weapons
  ;[1 1 1] LEVEL UP
  ;;[1 1 1] Upgrades
  (Variables|Stats|SetRange (+ (Variables|Stats|GetRange) 3.0))
  (Variables|Stats|SetReload%20Time (+ (Variables|Stats|GetReload%20Time) -0.1))
  (Variables|Stats|SetAim%20Delay (+ (Variables|Stats|GetAim%20Delay) -0.01))
  (Variables|Stats|SetPower (+ (Variables|Stats|GetPower) 1.0)))

(event Custom|CE_Armor
  ;[1 1 1] LEVEL UP
  ;;[1 1 1] Upgrades
  (Variables|Stats|SetArmor (+ (Variables|Stats|GetArmor) 1.0)))

(event EventBeginPlay
  (bind _returnvalue (Actor|GetActorOfClass "/Game/BP_Nobody.BP_Nobody_C"))
  (bind _output_get (Variables|Default|SetNOBODY _returnvalue))
  (Variables|AI|SetTarget _output_get)
  (CallFunction|CEPrint)
  (CallFunction|CEUPdate)
  (CallFunction|CESearch :!label _label)
  (Utilities|FlowControl|DoOnce false
    (:Completed
      (Utilities|FlowControl|Delay 0.2)
      (goto _label))))

(event EventDamage
  (params (Impact%20Point :type Vector :default "0, 0, 0"))
  (if (not (Variables|AI|Getseeking%20upgrade))
    (bind _output_get (Variables|Stats|SetHP (- (Variables|Stats|GetHP) (/ 1.0 (Variables|Stats|GetArmor)))))
    (if (<= _output_get 0.0)
      (CallFunction|CESplash)
      (Components|DestroyComponent (Variables|Collision|GetCapsuleComponent))
      (Rendering|SetVisibility (Variables|Default|GetWidget_Space) false false)
      (Components|Activation|Deactivate (Variables|Default|GetAIPerceptionStimuliSource))
      (Physics|SetSimulatePhysics (Variables|Character|GetMesh) true)
      (Physics|AddRadialForce (Variables|Character|GetMesh) Impact%20Point 1e+04 1e+04 "RIF_Constant" false)
      (Utilities|FlowControl|Delay 3.0)
      (Actor|DestroyActor)
      (else
        (CallFunction|CESplash)))))

(fn ConstructionScript)