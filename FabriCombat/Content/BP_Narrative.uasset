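; BP_Narrative drives story progression by playing narrative voice lines and updating the on-screen quest UI.
; BeginPlay and CE_Reset create a WDG_Narrative widget and add it to the viewport.
; The Narrative event stores an event index and switches to that step's sound array.
; CE_Narrative then plays a random 2D sound from the array and sends the next Quest entry to the widget.
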(event Custom|CE_Narrative
  (params (Sound%20Array :type Array%20of%20Sound%20Wave%20Object%20References))
  (Audio|PlaySound2D (Utilities|Array|Get(acopy) Sound%20Array (Math|Random|RandomInteger (Utilities|Array|Length Sound%20Array))) 1.0 1.0 0.0 0 0)
  (Default|NarrUIUpdate (Variables|Default|GetNarrWDG) (Utilities|Array|Get(acopy) (Variables|Default|GetQuest) (+ (Variables|Default|GetEvent) 1))))

(event Custom|CE_Reset
  (bind _returnvalue (UserInterface|CreateWidget "/Game/Widgets/WDG_Narrative.WDG_Narrative_C"))
  (bind _output_get (Variables|Default|SetNarrWDG _returnvalue))
  (UserInterface|Viewport|AddtoViewport _output_get 0))

(event EventBeginPlay
  (bind _returnvalue (UserInterface|CreateWidget "/Game/Widgets/WDG_Narrative.WDG_Narrative_C"))
  (bind _output_get (Variables|Default|SetNarrWDG _returnvalue))
  (UserInterface|Viewport|AddtoViewport _output_get 0))

(event EventNarrative
  (params (Event :type Integer))
  (bind _output_get (Variables|Default|SetEvent Event))
  (switch int _output_get
    (:0
      (CallFunction|CENarrative (Variables|Default|GetDIAL_0)))
    (:1
      (CallFunction|CENarrative (Variables|Default|GetDIAL_1)))
    (:2
      (CallFunction|CENarrative (Variables|Default|GetDIAL_2)))
    (:3
      (CallFunction|CENarrative (Variables|Default|GetDIAL_3)))
    (:4
      (CallFunction|CENarrative (Variables|Default|GetDIAL_4)))
    (:5
      (CallFunction|CENarrative (Variables|Default|GetDIAL_5)))
    (:6
      (CallFunction|CENarrative (Variables|Default|GetDIAL_6)))
    (:7
      (CallFunction|CENarrative (Variables|Default|GetDIAL_7)))
    (:8
      (CallFunction|CENarrative (Variables|Default|GetDIAL_8)))
    (:9
      (CallFunction|CENarrative (Variables|Default|GetDIAL_9)))
    (:10
      (CallFunction|CENarrative (Variables|Default|GetDIAL_10)))
    (:11
      (CallFunction|CENarrative (Variables|Default|GetDIAL_11)))
    (:12
      (CallFunction|CENarrative (Variables|Default|GetDIAL_12)))
    (:13
      (CallFunction|CENarrative (Variables|Default|GetDIAL_13)))
    (:14
      (CallFunction|CENarrative (Variables|Default|GetDIAL_14)))
    (:15
      (CallFunction|CENarrative (Variables|Default|GetDIAL_15)))
    (:16
      (CallFunction|CENarrative (Variables|Default|GetDIAL_16)))
    (:17
      (CallFunction|CENarrative (Variables|Default|GetDIAL_17)))
    (:18
      (CallFunction|CENarrative (Variables|Default|GetDIAL_18)))
    (:19
      (CallFunction|CENarrative (Variables|Default|GetDIAL_19)))
    (:20
      (CallFunction|CENarrative (Variables|Default|GetDIAL_20)))))

(fn ConstructionScript)