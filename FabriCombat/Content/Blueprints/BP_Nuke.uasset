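; BP_Nuke is a short-lived nuke explosion actor that plays its visual effect and damages whatever enters its area.
; On BeginPlay it spawns the NS_ACT_Nuke effect at its point light, and a timeline drives that light's intensity between a bright flash and zero.
; Any valid actor that begins overlapping the Box receives a DamageMessage.
; The actor destroys itself a few seconds after the timeline finishes.
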(event OnComponentBeginOverlap(Box)
  (params (OverlappedComponent :type Primitive%20Component%20Object%20Reference) (OtherActor :type Actor%20Object%20Reference) (OtherComp :type Primitive%20Component%20Object%20Reference) (OtherBodyIndex :type Integer) (bFromSweep :type Boolean) (SweepResult :type Hit%20Result%20Structure%20%28by%20ref%29))
  (Utilities|IsValid OtherActor
    (:Is%20Valid
      (Class|BPIInteract|Damage(Message) OtherActor "0, 0, 0" false))))

(event EventBeginPlay
  (Niagara|SpawnSystematLocation "/Game/Niagara/NS_ACT_Nuke.NS_ACT_Nuke" (Transformation|GetWorldLocation (Variables|Default|GetPointLight self)))
  (bind _newtrack_0 (Timeline|Timeline PlayFromStart)
    (:Update
      (Rendering|Components|Light|SetIntensity (Variables|Default|GetPointLight) (Math|Float|Lerp 5e+05 0.0 _newtrack_0)))
    (:Finished
      (Utilities|FlowControl|Delay 3.0)
      (Actor|DestroyActor))))

(fn ConstructionScript)