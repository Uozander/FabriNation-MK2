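; Alien enemy character that hunts citizens, melees them and takes typed damage.
; PawnSensing writes sighted BP_Citizen2 pawns to the Blackboard, while custom events run an AIMoveTo search/follow/fight loop whose own target-acquisition code is disconnected.
; Attacks sphere-trace ahead, damaging anything except fellow enemies.
; Resistance-scaled damage and speed-altering poison update a health-bar widget; death spawns splash and blood decals, plus an explosion for certain causes.
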(event OnSeePawn(PawnSensing)
  (params (Pawn :type Pawn%20Object%20Reference))
  (bind _self self)
  (bind _returnvalue (AI|GetAIController _self))
  (bind _returnvalue_2 (AI|GetBlackboard _returnvalue))
  (Utilities|IsValid _self
    (:Is%20Valid
      (if (== (Utilities|GetClass Pawn) "/Game/Blueprints/BP_Citizen2.BP_Citizen2_C")
        (AI|Components|Blackboard|SetValueasBool _returnvalue_2 (Utilities|Name|MakeLiteralName "SeenPlayer") true)
        (AI|Components|Blackboard|SetValueasObject _returnvalue_2 (Utilities|Name|MakeLiteralName "Target") Pawn)))))

(event OnTargetPerceptionUpdated(AIPerception)
  (params (Actor :type Actor%20Object%20Reference) (Stimulus :type AI%20Stimulus%20Structure))
  ;[0.4072 0.1559 0] DEP
)

(event Custom|CE_HealthUpdate
  (bind _aswdg_health_bar (Utilities|Casting|CastToWDG_Health_Bar (UserInterface|GetWidget (Variables|Default|GetWidget))))
  (Progress|SetPercent (Variables|/Game/Widgets/WDG_Health_Bar.WDG_Health_Bar_C|GetHealthBar _aswdg_health_bar) (/ (Variables|Default|GetHealth) 2e+01)))

(event Custom|CE_Search
  (if (Variables|Default|GetSeePlayer)
    (CallFunction|CEFollow)
    (else
      (Variables|Default|SetSearching true)
      (AI|AIMoveTo self (.RandomLocation (AI|Navigation|GetRandomReachablePointinRadius (Transformation|GetActorLocation self) 2e+03 0 0)) 0 1.5e+02 false
        (:OnSuccess
          _)
        (:OnFail
          _))
      (Variables|Default|SetSearching false)
      (Variables|Default|SetSeePlayer false)
      (CallFunction|CESearch))))

(event Custom|CE_Die
  (bind _self self)
  (bind _returnvalue (Transformation|GetActorLocation _self))
  (Game|SpawnActorfromClass "/Game/StarterContent/Blueprints/Blueprint_Effect_Explosion.Blueprint_Effect_Explosion_C" (Math|Transform|MakeTransform (Math|Vector|MakeVector (.x _returnvalue) (.y _returnvalue) (+ (.z _returnvalue) -1.8e+03)) "0, 0, 0" "3.000000,3.000000,3.000000") "Undefined" "MultiplyWithRoot" 0 0)
  (Variables|Default|SetDead true)
  (CallFunction|CESplash)
  (CallFunction|CEBlood)
  (Components|DestroyComponent (Variables|Collision|GetCapsuleComponent))
  (Actor|DestroyActor))

(event Custom|CE_Blood
  (bind _returnvalue (Transformation|GetActorLocation))
  (bind _outhit (Collision|LineTraceForObjects _returnvalue (- _returnvalue "0.000000,0.000000,200.000000") (Variables|Default|GetObject%20Types_Static) false 0 "None"))
  (switch int (Math|Random|RandomInteger 3)
    (:0
      (Rendering|Decal|SpawnDecalatLocation "/Game/Decals/MAT_Blood_Alien1.MAT_Blood_Alien1" (Math|Vector|MakeVector 1.0 (+ (* (Math|Random|RandomFloat) 1.2e+02) 9e+01) (+ (* (Math|Random|RandomFloat) 1.2e+02) 9e+01)) (.location _outhit) (Math|Rotator|MakeRotator (.roll (Math|Conversions|RotationFromXVector (.normal _outhit))) (.pitch (Math|Conversions|RotationFromXVector (.normal _outhit))) (* (Math|Random|RandomFloat) 3.6e+02)) 1e+01))
    (:1
      (Rendering|Decal|SpawnDecalatLocation "/Game/Decals/MAT_Blood_Alien2.MAT_Blood_Alien2" (Math|Vector|MakeVector 1.0 (+ (* (Math|Random|RandomFloat) 1.2e+02) 9e+01) (+ (* (Math|Random|RandomFloat) 1.2e+02) 9e+01)) (.location _outhit) (Math|Rotator|MakeRotator (.roll (Math|Conversions|RotationFromXVector (.normal _outhit))) (.pitch (Math|Conversions|RotationFromXVector (.normal _outhit))) (* (Math|Random|RandomFloat) 3.6e+02)) 1e+01))
    (:2
      (Rendering|Decal|SpawnDecalatLocation "/Game/Decals/MAT_Blood_Alien3.MAT_Blood_Alien3" (Math|Vector|MakeVector 1.0 (+ (* (Math|Random|RandomFloat) 1.2e+02) 9e+01) (+ (* (Math|Random|RandomFloat) 1.2e+02) 9e+01)) (.location _outhit) (Math|Rotator|MakeRotator (.roll (Math|Conversions|RotationFromXVector (.normal _outhit))) (.pitch (Math|Conversions|RotationFromXVector (.normal _outhit))) (* (Math|Random|RandomFloat) 3.6e+02)) 1e+01))))

(event Custom|CE_Follow
  (bind _target (Variables|Default|GetTarget))
  (AI|AIMoveTo self "0, 0, 0" (Variables|Default|GetTarget) 1.5e+02 false
    (:OnSuccess
      (Variables|Default|SetSeePlayer false)
      (Utilities|IsValid _target
        (:Is%20Valid
          (if (> (Transformation|GetDistanceTo _target self) 1.5e+02)
            (Rendering|Material|SetMaterial (Variables|Character|GetMesh) 0 "/Game/Characters/Mannequins/Materials/Instances/Quinn/MI_Quinn_01.MI_Quinn_01" :!label _label)
            (CallFunction|CESearch)
            (else
              (Rendering|Material|SetMaterial (Variables|Character|GetMesh) 0 "/Game/Materials/MAT_Red.MAT_Red")
              (Components|Movement|StopMovementImmediately (Variables|Character|GetCharacterMovement))
              (CallFunction|CEFight))))
        (:Is%20Not%20Valid
          (goto _label))))
    (:OnFail
      (Variables|Default|SetSeePlayer false)
      (CallFunction|CESearch))))

(event Custom|CE_Splash
  (bind _mesh (Variables|Character|GetMesh))
  (bind _returnvalue (Transformation|GetWorldLocation _mesh))
  (Niagara|SpawnSystematLocation "/Game/Meshes/CE_StickImpact_Alien.CE_StickImpact_Alien" (Math|Vector|MakeVector (.x _returnvalue) (.y _returnvalue) (+ (.z _returnvalue) 1e+02))))

(event Custom|CE_Fight
  (bind _returnvalue (Transformation|GetActorForwardVector))
  (bind _returnvalue_2 (Transformation|GetActorLocation))
  (bind _returnvalue_3 (* _returnvalue 1e+02))
  (bind _returnvalue_4 (- _returnvalue_2 "0.000000,0.000000,50.000000"))
  (bind _returnvalue_5 (+ _returnvalue_3 _returnvalue_4))
  (bind _outhits (Collision|MultiSphereTraceForObjects _returnvalue_5 _returnvalue_5 (* (Variables|Default|GetWindup) 2.4e+03) (Variables|Default|GetObject%20Types) false 0 "None"))
  (Niagara|SpawnSystematLocation "/Game/Niagara/NS_Slash.NS_Slash" _returnvalue_2 "0.000000,30.000000,0.000000" "0.200000,0.200000,0.200000")
  (Utilities|FlowControl|Sequence
    (:then_0
      (bind (_array_element_hitactor _array_element_impact_point) (|CollapseGraph_2 _outhits)
        (:LoopBody
          (if (not (== (Utilities|GetClass _array_element_hitactor) "BP_EnemyAI_C"))
            (Class|BPIInteract|Damage(Message) _array_element_hitactor _array_element_impact_point false)
            (AI|Components|Blackboard|SetValueasBool (AI|GetBlackboard (AI|GetAIController self)) (Utilities|Name|MakeLiteralName "SeenPlayer") false)))))
    (:then_1
      (Variables|Default|SetSeePlayer false)
      (CallFunction|CESearch))))

(event EventDamage
  (params (Impact%20Point :type Vector :default "0, 0, 0") (Missile? :type Boolean) (Damage%20Type :type Integer))
  (bind _self self)
  (bind _returnvalue (Transformation|GetActorLocation _self))
  (if (not (Variables|Default|GetDead))
    (switch int Damage%20Type
      (:0
        (bind _output_get (Variables|Default|SetHealth (- (Variables|Default|GetHealth) (/ 6.0 (+ (Variables|Default|GetRes_KIN) 1.0)))))
        (if (<= _output_get 0.0)
          (Variables|Default|SetDead true :!label _label)
          (CallFunction|CESplash)
          (CallFunction|CEBlood)
          (Components|DestroyComponent (Variables|Collision|GetCapsuleComponent))
          (Actor|DestroyActor)
          (else
            (CallFunction|CEHealthUpdate :!label _label_2))))
      (:1
        (bind _output_get_2 (Variables|Default|SetHealth (- (Variables|Default|GetHealth) (/ 2e+01 (+ (Variables|Default|GetRes_MIS) 1.0)))))
        (if (<= _output_get_2 0.0)
          (Game|SpawnActorfromClass "/Game/StarterContent/Blueprints/Blueprint_Effect_Explosion.Blueprint_Effect_Explosion_C" (Math|Transform|MakeTransform (Math|Vector|MakeVector (.x _returnvalue) (.y _returnvalue) (+ (.z _returnvalue) -1.8e+03)) "0, 0, 0" "3.000000,3.000000,3.000000") "Undefined" "MultiplyWithRoot" 0 0)
          (goto _label)
          (else
            (goto _label_2))))
      (:2
        (bind _output_get_3 (Variables|Default|SetHealth (- (Variables|Default|GetHealth) (/ 8.0 (+ (Variables|Default|GetRes_ENE) 1.0)))))
        (if (<= _output_get_3 0.0)
          (goto _label)
          (else
            (goto _label_2)))))))

(event EventPoison
  (bind _charactermovement (Variables|Character|GetCharacterMovement))
  (Variables|/Script/Engine.CharacterMovementComponent|SetMaxWalkSpeed _charactermovement 6e+02)
  (bind _output_get (Variables|Default|SetHealth (- (Variables|Default|GetHealth) 0.1)))
  (if (<= _output_get 0.0)
    (CallFunction|CEDie)
    (else
      (CallFunction|CEHealthUpdate)
      (Utilities|FlowControl|RetriggerableDelay 3.0)
      (Variables|/Script/Engine.CharacterMovementComponent|SetMaxWalkSpeed _charactermovement 6e+03))))

(event EventBeginPlay
  (Components|Activation|Activate (Variables|Default|GetAIPerceptionStimuliSource) false)
  (Components|Activation|Activate (Variables|Default|GetAIPerception) false))

(fn ConstructionScript)