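; BP_Bombard is an artillery actor that, ten seconds after BeginPlay, fires a rapid barrage of BP_Blaster2 projectiles from its Sphere until Rounds runs out.
; About three quarters of shots aim at a random BP_EnemyAI; the rest scatter, mostly downward.
; Aimed shots send DamageMessage after a short delay, independent of projectile impact.
; Each random index is re-rolled, so aimed and damaged enemies can differ.
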(event Custom|CE_Blast
  (bind _returnvalue (Game|SpawnActorfromClass "/Game/Blueprints/BP_Blaster2.BP_Blaster2_C" (Math|Transform|MakeTransform (Transformation|GetWorldLocation (Variables|Default|GetSphere)) "0, 0, 0" "1.000000,1.000000,1.000000") "Undefined" "MultiplyWithRoot" 0 0))
  (Physics|AddImpulse (Variables|/Game/Blueprints/BP_Blaster2.BP_Blaster2_C|GetSphere _returnvalue) (Variables|Default|GetImpulse) "None" true))

(event Custom|CE_Pick_Target
  (bind _out_actors (Variables|Default|GetOut%20Actors))
  (bind _returnvalue (Utilities|Array|Length _out_actors))
  (bind _returnvalue_2 (Math|Random|RandomInteger _returnvalue))
  (bind _output (Utilities|Array|Get(acopy) _out_actors _returnvalue_2))
  (Utilities|IsValid _output
    (:Is%20Valid
      (bind _output_get (Variables|Default|SetRotation (Math|Rotator|FindLookatRotation (Transformation|GetWorldLocation (Variables|Default|GetSphere)) (Transformation|GetActorLocation _output))))
      (Variables|Default|SetImpulse (* (Math|Rotator|GetRotationXVector _output_get) 1.5e+04))
      (Utilities|FlowControl|Delay 0.2)
      (Class|BPIInteract|Damage(Message) _output "0, 0, 0" false))
    (:Is%20Not%20Valid
      (Utilities|FlowControl|DoOnce false
        (:Completed
          (CallFunction|CEPickTarget))))))

(event EventBeginPlay
  (Utilities|FlowControl|Delay 1e+01)
  (bind _outactors (Actor|GetAllActorsOfClass "/Game/Blueprints/BP_EnemyAI.BP_EnemyAI_C"))
  (Variables|Default|SetOut%20Actors _outactors)
  (if (> (Variables|Default|GetRounds) 0) :!label _label
    (if (Math|Random|RandomBool)
      (CallFunction|CEPickTarget :!label _label_2)
      (CallFunction|CEBlast)
      (elif (Math|Random|RandomBool)
        (goto _label_2)
        (else
          (Variables|Default|SetImpulse (Math|Vector|MakeVector (* (- (Math|Random|RandomFloat) 0.05) 1e+03) (* (- (Math|Random|RandomFloat) 0.05) 1e+03) (* (Math|Random|RandomFloat) -5e+02)))
          (CallFunction|CEBlast))))
    (Utilities|FlowControl|Delay 0.0001)
    (Variables|Default|SetRounds (- (Variables|Default|GetRounds) 1))
    (goto _label)))

(fn ConstructionScript)