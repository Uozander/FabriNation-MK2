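; BP_Wall is a wall that gets broken down while enemy AI or citizens touch it.
; Overlapping its R component with a BP_EnemyAI or BP_Citizen2 starts a looping Delay that steadily shrinks the mesh's Z scale, destroying the actor at a minimum height.
; The loop stops, leaving the wall partly lowered, once neither class remains overlapping.
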(event OnComponentBeginOverlap(r)
  (params (OverlappedComponent :type Primitive%20Component%20Object%20Reference) (OtherActor :type Actor%20Object%20Reference) (OtherComp :type Primitive%20Component%20Object%20Reference) (OtherBodyIndex :type Integer) (bFromSweep :type Boolean) (SweepResult :type Hit%20Result%20Structure%20%28by%20ref%29))
  (if (or (== (Utilities|GetClass OtherActor) "/Game/Blueprints/BP_EnemyAI.BP_EnemyAI_C") (== (Utilities|GetClass OtherActor) "/Game/Blueprints/BP_Citizen2.BP_Citizen2_C"))
    (Variables|Default|SetBreaking true)
    (if (Variables|Default|GetBreaking) :!label _label
      (Transformation|SetRelativeTransform (Variables|Default|GetStaticMesh) (Math|Transform|MakeTransform "0, 0, 0" "0, 0, 0" (Math|Vector|MakeVector 3.893428 1.0 (+ (Variables|Default|GetNew%20Transform%20Scale%20Z) -0.05))) false false)
      (Variables|Default|SetNew%20Transform%20Scale%20Z (+ (Variables|Default|GetNew%20Transform%20Scale%20Z) -0.05))
      (Utilities|FlowControl|Delay 0.05)
      (if (<= (Variables|Default|GetNew%20Transform%20Scale%20Z) 2.0)
        (Actor|DestroyActor)
        (else
          (goto _label))))))

(event OnComponentEndOverlap(r)
  (params (OverlappedComponent :type Primitive%20Component%20Object%20Reference) (OtherActor :type Actor%20Object%20Reference) (OtherComp :type Primitive%20Component%20Object%20Reference) (OtherBodyIndex :type Integer))
  (bind _r (Variables|Default|Getr))
  (if (and (Utilities|Array|IsEmpty (Collision|GetOverlappingActors _r "/Game/Blueprints/BP_EnemyAI.BP_EnemyAI_C" :!class /Script/Engine.PrimitiveComponent)) (Utilities|Array|IsEmpty (Collision|GetOverlappingActors _r "/Game/Blueprints/BP_Citizen2.BP_Citizen2_C" :!class /Script/Engine.PrimitiveComponent)))
    (Variables|Default|SetBreaking false)))

(fn ConstructionScript)