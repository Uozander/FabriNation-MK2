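; BP_Tower is a cannon tower that fires once at each BP_EnemyAI actor as it enters its Box trigger.
; On overlap, it snaps the Cannon toward the enemy with a pitch offset, plays a fire sound and sends a DamageMessage directly, without a projectile.
; The shot also starts a Timeline whose event track uses a FlipFlop to alternate two pairs of muzzle flashes, hiding all four when finished.
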(event OnComponentBeginOverlap(Box)
  (params (OverlappedComponent :type Primitive%20Component%20Object%20Reference) (OtherActor :type Actor%20Object%20Reference) (OtherComp :type Primitive%20Component%20Object%20Reference) (OtherBodyIndex :type Integer) (bFromSweep :type Boolean) (SweepResult :type Hit%20Result%20Structure%20%28by%20ref%29))
  (bind _returnvalue (Transformation|GetActorLocation OtherActor))
  (bind _self self)
  (bind _returnvalue_2 (Transformation|GetActorLocation _self))
  (bind _returnvalue_3 (Math|Rotator|FindLookatRotation _returnvalue_2 _returnvalue))
  (if (== "/Game/Blueprints/BP_EnemyAI.BP_EnemyAI_C" (Utilities|GetClass OtherActor))
    (Transformation|SetWorldRotation (Variables|Default|GetCannon) (Math|Rotator|MakeRotator (.roll _returnvalue_3) (+ (.pitch _returnvalue_3) -9e+01) (.yaw _returnvalue_3)) false false)
    (Audio|PlaySoundatLocation "/Game/Sounds/cannon-fire-161072.cannon-fire-161072" (Transformation|GetActorLocation) "0, 0, 0" 0.5 1.0 0.0 0 0 0 0)
    (CallFunction|CEMuzzleShot)
    (Utilities|IsValid OtherActor
      (:Is%20Valid
        (Class|BPIInteract|Damage(Message) OtherActor "0, 0, 0" false)))))

(event Custom|CE_MuzzleShot
  (bind _muzzle_flash (Variables|Default|GetMuzzle_Flash))
  (bind _muzzle_flash3 (Variables|Default|GetMuzzle_Flash3))
  (Timeline|Timeline PlayFromStart
    (:Finished
      (Rendering|SetVisibility (Variables|Default|GetMuzzle_Flash1) false false))
    (:NewTrack_1
      (Utilities|FlowControl|FlipFlop
        (:A
          (Rendering|SetVisibility _muzzle_flash3 true false)
          (Rendering|SetVisibility _muzzle_flash false false))
        (:B
          (Rendering|SetVisibility _muzzle_flash true false)
          (Rendering|SetVisibility _muzzle_flash3 false false))))))

(fn ConstructionScript)