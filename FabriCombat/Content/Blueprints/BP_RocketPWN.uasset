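; BP_RocketPWN is a rocket pawn that the player possesses while it flies at a random enemy.
; CE_Launch chains timeline lerps: a forward climb, a run at a random BP_EnemyAI, then a re-aimed final leg that damages it.
; If the target becomes invalid before that leg, the rocket dives to a fixed height and spawns an explosion effect.
; Both endings call CEBoom, hide the mesh, repossess BP_TopDownCharacter and destroy the rocket.
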(event Custom|CE_Launch
  (params (Forward%20Vector :type Vector))
  (Variables|Default|SetForward%20Vector Forward%20Vector)
  (Transformation|SetActorRotation self (Math|Rotator|FindLookatRotation (Variables|Default|GetLock_Location) (+ (Variables|Default|GetLock_Location) (+ (* (Variables|Default|GetForward%20Vector) 4e+03) "0.000000,0.000000,4000.000000"))))
  (bind _newtrack_0 (Timeline|Timeline PlayFromStart)
    (:Update
      (Transformation|SetActorLocation self (Math|Vector|Lerp(Vector) (Variables|Default|GetLock_Location) (+ (Variables|Default|GetLock_Location) (+ (* (Variables|Default|GetForward%20Vector) 4e+03) "0.000000,0.000000,4000.000000")) _newtrack_0) false false))
    (:Finished
      (Utilities|FlowControl|Delay 0.1)
      (Variables|Default|SetLock_Location (Transformation|GetWorldLocation (Variables|Default|GetStaticMesh)))
      (bind _outactors (Actor|GetAllActorsOfClass "/Game/Blueprints/BP_EnemyAI.BP_EnemyAI_C"))
      (Utilities|IsValid (Utilities|Array|Get(acopy) _outactors (Math|Random|RandomInteger (Utilities|Array|Length _outactors))) :!label _label
        (:Is%20Valid
          (bind _output_get (Variables|Default|SetTarget (Utilities|Array|Get(acopy) _outactors (Math|Random|RandomInteger (Utilities|Array|Length _outactors)))))
          (Variables|Default|SetTarget_Location (Transformation|GetActorLocation _output_get))
          (Transformation|SetActorRotation (Math|Rotator|FindLookatRotation (Variables|Default|GetLock_Location) (Variables|Default|GetTarget_Location)))
          (bind _newtrack_0_2 (Timeline|Timeline_0 PlayFromStart)
            (:Update
              (Transformation|SetActorLocation self (Math|Vector|Lerp(Vector) (Variables|Default|GetLock_Location) (Variables|Default|GetTarget_Location) _newtrack_0_2) false false))
            (:Finished
              (Variables|Default|SetLock_Location (Transformation|GetWorldLocation (Variables|Default|GetStaticMesh)))
              (Utilities|IsValid (Variables|Default|GetTarget)
                (:Is%20Valid
                  (Variables|Default|SetTarget_Location (Transformation|GetActorLocation (Variables|Default|GetTarget)))
                  (Transformation|SetActorRotation (Math|Rotator|FindLookatRotation (Variables|Default|GetLock_Location) (Variables|Default|GetTarget_Location)))
                  (bind _newtrack_0_3 (Timeline|Timeline_1 PlayFromStart)
                    (:Update
                      (Transformation|SetActorLocation self (Math|Vector|Lerp(Vector) (Variables|Default|GetLock_Location) (Variables|Default|GetTarget_Location) _newtrack_0_3) false false))
                    (:Finished
                      (Utilities|IsValid (Variables|Default|GetTarget)
                        (:Is%20Valid
                          (Default|Damage (Variables|Default|GetTarget) "0, 0, 0" true 1))
                        (:Is%20Not%20Valid
                          _))
                      (CallFunction|CEBoom)
                      (Rendering|SetVisibility (Variables|Default|GetStaticMesh) false true)
                      (Transformation|SetRelativeRotation (Variables|Default|GetSphere) "-40.000000,0.000000,0.000000" false false)
                      (Utilities|FlowControl|Delay 2.0)
                      (bind _returnvalue (Actor|GetActorOfClass "/Game/TopDown/Blueprints/BP_TopDownCharacter.BP_TopDownCharacter_C"))
                      (Pawn|Possess (Game|GetPlayerController 0) _returnvalue)
                      (Actor|DestroyActor))))
                (:Is%20Not%20Valid
                  (Transformation|SetActorRotation (Math|Rotator|FindLookatRotation (Variables|Default|GetLock_Location) (Math|Vector|MakeVector (.X (Math|Vector|BreakVector (Variables|Default|GetLock_Location))) (.Y (Math|Vector|BreakVector (Variables|Default|GetLock_Location))) -5.5e+02)))
                  (bind _newtrack_0_4 (Timeline|Timeline_2 PlayFromStart)
                    (:Update
                      (Transformation|SetActorLocation self (Math|Vector|Lerp(Vector) (Variables|Default|GetLock_Location) (Math|Vector|MakeVector (.X (Math|Vector|BreakVector (Variables|Default|GetLock_Location))) (.Y (Math|Vector|BreakVector (Variables|Default|GetLock_Location))) -5.5e+02) _newtrack_0_4) false false))
                    (:Finished
                      (CallFunction|CEBoom)
                      (Rendering|SetVisibility (Variables|Default|GetStaticMesh) false true)
                      (Game|SpawnActorfromClass "/Game/StarterContent/Blueprints/Blueprint_Effect_Explosion.Blueprint_Effect_Explosion_C" (Math|Transform|MakeTransform (Transformation|GetWorldLocation (Variables|Default|GetStaticMesh)) "0, 0, 0" "1.000000,1.000000,1.000000") "Undefined" "MultiplyWithRoot" 0 0)
                      (Transformation|SetRelativeRotation (Variables|Default|GetSphere) "-40.000000,0.000000,0.000000" false false)
                      (Utilities|FlowControl|Delay 3.0)
                      (bind _returnvalue_2 (Actor|GetActorOfClass "/Game/TopDown/Blueprints/BP_TopDownCharacter.BP_TopDownCharacter_C"))
                      (Pawn|Possess (Game|GetPlayerController 0) _returnvalue_2)
                      (Actor|DestroyActor))))))))
        (:Is%20Not%20Valid
          (Utilities|FlowControl|Delay 0.01)
          (goto _label))))))

(event Custom|CE_Boom
  (Audio|PlaySoundatLocation "/Game/Sounds/explosion-47821.explosion-47821" (Transformation|GetActorLocation) "0, 0, 0" 0.1 1.0 0.4 0 0 0 0))

(event EventBeginPlay
  (Variables|Default|SetLock_Location (Transformation|GetWorldLocation (Variables|Default|GetStaticMesh)))
  (Utilities|FlowControl|Delay 0.2)
  (Components|Activation|Activate (Variables|Default|GetAudio) false)
  (Pawn|Possess (Game|GetPlayerController 0) self))

(fn ConstructionScript)