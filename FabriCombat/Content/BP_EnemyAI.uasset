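; Enemy AI character that wanders to random reachable points, chases perceived actors with a matching tag and attacks them in melee.
; AI Perception sets the target, and AIMoveTo drives the search and follow loop.
; Within range it turns red, swings via timeline, then sphere-traces to send damage and spawn impact effects, both trace and effect scaled by Windup.
; When damaged itself, it ragdolls with a radial force and is destroyed after a delay.
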(event OnSeePawn(PawnSensing)
  (params (Pawn :type Pawn%20Object%20Reference)))

(event OnPerceptionUpdated(AIPerception)
  (params (UpdatedActors :type Array%20of%20Actor%20Object%20References)))

(event OnTargetPerceptionInfoUpdated(AIPerception)
  (params (UpdateInfo :type Actor%20Perception%20Update%20Info%20Structure%20%28by%20ref%29)))

(event OnTargetPerceptionUpdated(AIPerception)
  (params (Actor :type Actor%20Object%20Reference) (Stimulus :type AI%20Stimulus%20Structure))
  (if (Actor|ActorHasTag Actor (Variables|Default|GetTag))
    (Utilities|IsValid Actor
      (:Is%20Valid
        (Variables|Default|SetTarget Actor)
        (if (> (Transformation|GetDistanceTo (Variables|Default|GetTarget) self) 7e+01)
          (Rendering|Material|SetMaterial (Variables|Character|GetMesh) 0 "/Game/Characters/Mannequins/Materials/Instances/Quinn/MI_Quinn_01.MI_Quinn_01"))
        (Variables|Default|SetSeePlayer true)
        (CallFunction|CEFollow)))))

(event Custom|CE_Swing
  (bind _newtrack_2 (Timeline|Timeline_0 PlayFromStart)
    (:Update
      (Transformation|SetRelativeRotation (Variables|Default|Getrr) (Math|Rotator|MakeRotator 0.0 (Math|Float|Lerp 0.0 -1.1e+02 _newtrack_2) 0.0) false false))
    (:Finished
      (Transformation|SetRelativeRotation (Variables|Default|Getrr) (Math|Rotator|MakeRotator 0.0 0.0 0.0) false false))))

(event Custom|CE_Search
  (if (Variables|Default|GetSeePlayer)
    (CallFunction|CEFollow)
    (else
      (Variables|Default|SetSearching true)
      (AI|AIMoveTo self (.RandomLocation (AI|Navigation|GetRandomReachablePointinRadius (Transformation|GetActorLocation self) 2e+03 0 0)) 0 1.5e+02 false
        (:OnSuccess
          _)
        (:OnFail
          _))
      (Variables|Default|SetSearching false)
      (Variables|Default|SetSeePlayer false)
      (CallFunction|CESearch))))

(event Custom|CE_Windup
  (bind _newtrack_2 (Timeline|Timeline PlayFromStart)
    (:Update
      (Variables|Default|SetWindup _newtrack_2)
      (Transformation|SetRelativeRotation (Variables|Default|Getrr) (Math|Rotator|MakeRotator 0.0 (Math|Float|Lerp 0.0 55.0 _newtrack_2) 0.0) false false))))

(event Custom|CE_Follow
  (bind _returnvalue (Transformation|GetActorLocation))
  (bind _self self)
  (bind _target (Variables|Default|GetTarget))
  (bind _windup (Variables|Default|GetWindup))
  (bind _returnvalue_2 (Transformation|GetActorForwardVector _self))
  (bind _returnvalue_3 (* _windup 25.0))
  (bind _returnvalue_4 (- _returnvalue "0.000000,0.000000,50.000000"))
  (bind _returnvalue_5 (* _returnvalue_2 1e+02))
  (bind _returnvalue_6 (+ _returnvalue_5 _returnvalue_4))
  (AI|AIMoveTo self (Transformation|GetActorLocation (Variables|Default|GetTarget)) 0 1.5e+02 false
    (:OnSuccess
      (Variables|Default|SetSeePlayer false)
      (Utilities|IsValid _target
        (:Is%20Valid
          (if (> (Transformation|GetDistanceTo _target self) 1.5e+02)
            (Rendering|Material|SetMaterial (Variables|Character|GetMesh) 0 "/Game/Characters/Mannequins/Materials/Instances/Quinn/MI_Quinn_01.MI_Quinn_01" :!label _label)
            (CallFunction|CESearch)
            (else
              (Rendering|Material|SetMaterial (Variables|Character|GetMesh) 0 "/Game/MAT_Red.MAT_Red")
              (Components|Movement|StopMovementImmediately (Variables|Character|GetCharacterMovement))
              (CallFunction|CESwing)
              (Utilities|FlowControl|Delay 0.25)
              (bind _outhits (Collision|MultiSphereTraceForObjects _returnvalue_6 _returnvalue_6 (* _windup 6e+02) (Variables|Default|GetObject%20Types) false 0 "ForDuration"))
              (bind _array_element_hitactor (|CollapseGraph_2 _outhits)
                (:LoopBody
                  (Class|NewInterface|Damage(Message) _array_element_hitactor _returnvalue_6)
                  (Niagara|SpawnSystematLocation "/Game/CE_StickImpact.CE_StickImpact" _returnvalue_6 "0, 0, 0" (Math|Vector|MakeVector _returnvalue_3 _returnvalue_3 _returnvalue_3))
                  (Variables|Default|SetSeePlayer false)
                  (CallFunction|CESearch))))))
        (:Is%20Not%20Valid
          (goto _label))))
    (:OnFail
      (Variables|Default|SetSeePlayer false)
      (CallFunction|CESearch))))

(event EventBeginPlay
  (Components|Activation|Activate (Variables|Default|GetAIPerceptionStimuliSource) false)
  (Components|Activation|Activate (Variables|Default|GetAIPerception) false)
  (CallFunction|CESearch :!label _label)
  (Utilities|FlowControl|DoOnce false
    (:Completed
      (Utilities|FlowControl|Delay 0.2)
      (goto _label))))

(event EventDamage
  (params (Impact%20Point :type Vector :default "0, 0, 0"))
  (Physics|SetSimulatePhysics (Variables|Character|GetMesh) true)
  (Physics|AddRadialForce (Variables|Character|GetMesh) Impact%20Point 1e+04 1e+04 "RIF_Constant" false)
  (Collision|SetCollisionEnabled (Variables|Collision|GetCapsuleComponent) "NoCollision")
  (Utilities|FlowControl|Delay 3.0)
  (Actor|DestroyActor))

(fn ConstructionScript)